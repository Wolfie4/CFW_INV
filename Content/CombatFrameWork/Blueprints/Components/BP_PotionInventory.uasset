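; Actor component that tracks a potion count and handles drinking potions to restore the owner's health, stamina or mana through BP_Stats.
; DrinkPotion checks the count, decrements it, restores health, calls CallUpdatePotionAmount and empties the glass mesh.
; Stamina and mana variants share that count and restore amount but skip those checks and updates.
; SpawnPotion attaches a BP_Potion to a character mesh socket, DespawnPotion destroys it, and Bonfire only calls CallUpdatePotionAmount.
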(event `Drink Stamina Potion`
  ;[1 1 1] Doesnt get called on the animation. Maybe try addinga  New Emum (E_ConsumableType) with a switcher that checks what the potion is before calling on the heal player
  (`/Engine/EditorBlueprintResources/StandardMacros.DecrementInt` (`self.PotionQuantity`)
    (:`  `
      (`/Game/CombatFrameWork/Blueprints/Components/BP_Stats.RestorePlayerStamina` (`Actor.GetComponentByClass` (`self.GetOwner`) "/Game/CombatFrameWork/Blueprints/Components/BP_Stats.BP_Stats_C") (`self.PotionRestoreAmount`)))))

(event `Drink Mana Potion`
  ;[1 1 1] Doesnt get called on the animation. Maybe try addinga  New Emum (E_ConsumableType) with a switcher that checks what the potion is before calling on the heal player
  (`/Engine/EditorBlueprintResources/StandardMacros.DecrementInt` (`self.PotionQuantity`)
    (:`  `
      (`/Game/CombatFrameWork/Blueprints/Components/BP_Stats.RestorePlayerMana` (`Actor.GetComponentByClass` (`self.GetOwner`) "/Game/CombatFrameWork/Blueprints/Components/BP_Stats.BP_Stats_C") (`self.PotionRestoreAmount`)))))

(event `Drink Potion`
  (bind _potionquantity (`self.PotionQuantity`))
  (bind _potionmesh (`self.PotionMesh`))
  (if (> _potionquantity 0)
    (bind _result (`/Engine/EditorBlueprintResources/StandardMacros.DecrementInt` _potionquantity)
      (:`  `
        (`KismetSystemLibrary.PrintString` (`KismetStringLibrary.Conv_IntToString` _result))
        (`/Game/CombatFrameWork/Blueprints/Components/BP_Stats.RestorePlayerHealth` (`Actor.GetComponentByClass` (`self.GetOwner`) "/Game/CombatFrameWork/Blueprints/Components/BP_Stats.BP_Stats_C") (`self.PotionRestoreAmount`))
        (`self.UpdatePotionAmount`)
        (`/Engine/EditorBlueprintResources/StandardMacros.IsValid` _potionmesh
          (:`Is Valid`
            (`/Game/CombatFrameWork/Blueprints/BP_Potion.EmptyGlass` _potionmesh)))))))

(event `Spawn Potion`
  (bind _returnvalue (`self.GetOwner`))
  (bind _returnvalue_2 (`|SpawnActorFromClass` "/Game/CombatFrameWork/Blueprints/BP_Potion.BP_Potion_C" (`Actor.GetTransform` _returnvalue) "AlwaysSpawn" "MultiplyWithRoot" null null))
  (bind _output_get (set `self.PotionMesh` _returnvalue_2))
  (`Actor.K2_AttachToComponent` _output_get (`Character.Mesh` (cast `Character` _returnvalue :!pure true)) (`self.Socket Name`) "SnapToTarget" "SnapToTarget" "SnapToTarget" true))

(event `Despawn Potion`
  (bind _potionmesh (`self.PotionMesh`))
  (`/Engine/EditorBlueprintResources/StandardMacros.IsValid` _potionmesh
    (:`Is Valid`
      (`Actor.K2_DestroyActor` _potionmesh))))

(event `Bonfire`
  (`self.UpdatePotionAmount`))