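; Elven bow weapon Blueprint in the combat framework that handles drawing and releasing the bowstring.
; DrawString plays a timeline that drives AimAlpha between 0 and 1, and ReleaseString reverses that same timeline to ease it back.
; BeginPlay, overlap and Tick are disabled stubs, and the construction script only calls its parent.
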(event `DrawString`
  (bind (_direction _drawalpha) (`Timeline|BowTimeline` :!label _label)
    (:`Update`
      (set `self.AimAlpha` (`KismetMathLibrary.Lerp` 0.0 1.0 _drawalpha)))))

(event `Release String`
  (goto _label :!via `Reverse`))

(fn `UserConstructionScript`
  (`parent.UserConstructionScript`))