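; Actor component that persists a campfire location in a save game slot.
; On BeginPlay it loads the existing Campfire save, or creates one seeded with the owner's current location and writes it to the slot.
; The UpdateCampfire event stores a supplied location in the cached save object and saves it immediately, if that object is valid.
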(event `self.ReceiveBeginPlay`
  (bind _returnvalue (`GameplayStatics.DoesSaveGameExist` "Campfire"))
  (if _returnvalue
    (bind _returnvalue_2 (`GameplayStatics.LoadGameFromSlot` "Campfire"))
    (bind _asbp_campfire_save (cast `/Game/CombatFrameWork/Blueprints/Save/BP_CampfireSave` _returnvalue_2))
    (set `self.CampfireSave` _asbp_campfire_save)
    (else
      (bind _returnvalue_3 (`GameplayStatics.CreateSaveGameObject` "/Game/CombatFrameWork/Blueprints/Save/BP_CampfireSave.BP_CampfireSave_C"))
      (bind _output_get (set `self.CampfireSave` _returnvalue_3))
      (set `/Game/CombatFrameWork/Blueprints/Save/BP_CampfireSave.CampfireLocation` (`Actor.K2_GetActorLocation` (`self.GetOwner`)) _output_get)
      (`GameplayStatics.SaveGameToSlot` _output_get "Campfire"))))

(event `UpdateCampfire`
  (params (Location :type "Vector Structure"))
  (bind _campfiresave (`self.CampfireSave`))
  (`/Engine/EditorBlueprintResources/StandardMacros.IsValid` (`self.CampfireSave`)
    (:`Is Valid`
      (set `/Game/CombatFrameWork/Blueprints/Save/BP_CampfireSave.CampfireLocation` Location _campfiresave)
      (`GameplayStatics.SaveGameToSlot` _campfiresave "campfire"))))