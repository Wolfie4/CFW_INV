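; Anim notify state that spawns a weapon trail particle effect on a combat character's main weapon during an animation.
; On begin, it gets the weapon mesh through the BP_CombatCharacter owner's BPCombat and attaches the emitter at the start socket with SnapToTarget.
; It passes a look-at rotation from the start socket toward the end socket.
; The end event only returns true, leaving the emitter untouched.
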(fn `Received_NotifyBegin`
  (params (MeshComp :type "SkeletalMeshComponent Object Reference") (Animation :type "AnimSequenceBase Object Reference") (TotalDuration :type "Float (single-precision)") (EventReference :type "AnimNotifyEventReference Structure (by ref)"))
  (returns (ReturnValue :type Boolean))
  (locals (CachedWeaponMesh :type "SceneComponent Object Reference"))
  (bind _staticmesh (`/Game/CombatFrameWork/Blueprints/Equipment/BP_BaseEquipment.StaticMesh` (`/Game/CombatFrameWork/Blueprints/Components/BP_Combat.MainWeapon` (`/Game/ThirdPerson/Blueprints/BP_CombatCharacter.BP_Combat` (cast `/Game/ThirdPerson/Blueprints/BP_CombatCharacter` (`ActorComponent.GetOwner` MeshComp) :!pure true)))))
  (`GameplayStatics.SpawnEmitterAttached` (`self.TrailParticleSystem`) _staticmesh (`self.WeaponAttachStartSocketName`) (`SceneComponent.K2_GetComponentLocation` _staticmesh) (`KismetMathLibrary.FindLookAtRotation` (`SceneComponent.GetSocketLocation` _staticmesh (`self.WeaponAttachStartSocketName`)) (`SceneComponent.GetSocketLocation` _staticmesh (`self.WeaponAttachEndSocketName`))) (1.0 1.0 1.0) "SnapToTarget")
  (return true))

(fn `Received_NotifyEnd`
  (params (MeshComp :type "SkeletalMeshComponent Object Reference") (Animation :type "AnimSequenceBase Object Reference") (EventReference :type "AnimNotifyEventReference Structure (by ref)"))
  (returns (ReturnValue :type Boolean))
  (return true))