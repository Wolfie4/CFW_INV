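; BP_ArrowBase is a combat arrow actor that flies as a projectile and deals point damage on hit.
; FireArrow adds a projectile movement component at runtime, sets scaled velocity and gravity, and attaches a Niagara trail.
; When the box overlaps a non-owner actor, it removes movement and trail, triggers VFX, applies damage, and destroys itself after a delay.
; Hit components tagged "Head" take double damage.
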(event `FireArrow`
  (params (Velocity :type "Vector Structure"))
  (bind _returnvalue (`AddComponent|NODE_AddProjectileMovementComponent-0`))
  (bind _output_get (set `self.ProjectileRef` _returnvalue))
  (set `MovementComponent.Velocity` (* Velocity (`self.ArrowStrength`)) _output_get)
  (set `ProjectileMovementComponent.ProjectileGravityScale` (`self.Projectile Gravity Scale`) _output_get)
  (bind _returnvalue_2 (`NiagaraFunctionLibrary.SpawnSystemAttached` (`self.ArrowTrail_NS`) (`self.Arrow`) "None" (0.0 0.0 0.0) (struct) "SnapToTarget"))
  (set `self.SystemRef` _returnvalue_2))

(event `self.Box.OnComponentBeginOverlap`
  (params (OverlappedComponent :type "PrimitiveComponent Object Reference") (OtherActor :type "Actor Object Reference") (OtherComp :type "PrimitiveComponent Object Reference") (OtherBodyIndex :type Integer) (bFromSweep :type Boolean) (SweepResult :type "HitResult Structure (by ref)"))
  (if (!= OtherActor (`self.GetOwner`))
    (bind _projectileref (`self.ProjectileRef`)
      (:`then`
        (`ActorComponent.K2_DestroyComponent` _projectileref)
        (bind _systemref (`self.SystemRef`)
          (:`then`
            (`ActorComponent.K2_DestroyComponent` _systemref)
            (`self.VFX`)
            (`GameplayStatics.ApplyPointDamage` OtherActor (select `bool` (`ActorComponent.ComponentHasTag` (`.HitComponent` (`GameplayStatics.BreakHitResult` SweepResult)) "Head") :`false` (`self.ArrowBaseDamage`) :`true` (* (`self.ArrowBaseDamage`) 2.0) :!type "Float (single-precision)") (`SceneComponent.GetForwardVector` (`self.Arrow`)) SweepResult (`self.GetInstigatorController` (`self.GetOwner`)) self "/Game/CombatFrameWork/Blueprints/Damage/BP_DamageType.BP_DamageType_C")
            (`KismetSystemLibrary.Delay` 5.0)
            (`self.K2_DestroyActor`))
          (:`else`)))
      (:`else`))))

(fn `UserConstructionScript`)