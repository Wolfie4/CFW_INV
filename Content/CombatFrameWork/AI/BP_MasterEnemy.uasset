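; Base enemy character for the combat framework, handling attacks, damage, targeting and death.
; Stats and state components drive stamina-costed random attack montages, damage multipliers and the health bar.
; Point damage reports to AI senses, plays attacker-based sound, blood and directional hit reactions chosen by relative yaw, with optional stun.
; Parries enable ripostes, a blackboard flag enables stealth kills, and normal death ragdolls the mesh before delayed destruction.
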(event `self.ReceiveBeginPlay`
  (`self.Create Health bar`))

(event `self.ReceivePointDamage`
  (params (Damage :type "Float (single-precision)") (DamageType :type "DamageType Object Reference") (HitLocation :type "Vector Structure") (HitNormal :type "Vector Structure") (HitComponent :type "PrimitiveComponent Object Reference") (BoneName :type Name) (ShotFromDirection :type "Vector Structure") (InstigatedBy :type "Controller Object Reference") (DamageCauser :type "Actor Object Reference") (HitInfo :type "HitResult Structure (by ref)"))
  (bind _returnvalue (`Controller.K2_GetPawn` InstigatedBy))
  (bind (_asbp_combat_character _bsuccess) (cast `/Game/ThirdPerson/Blueprints/BP_CombatCharacter` _returnvalue :!pure true))
  (`/Game/CombatFrameWork/Blueprints/Components/BP_Stats.Take Damage` (`self.BP_Stats`) Damage)
  (if (not (`/Game/CombatFrameWork/Blueprints/Components/BP_State.is Current State Equal To Any` (`self.BP_State`) (struct :`GameplayTags` (struct :`(TagName` "Player.State.Death")))))
    (`AISense_Damage.ReportDamageEvent` self _returnvalue Damage HitLocation)
    ;[0.06965 1 0] Might be working no errors after branch added. maybe find better way still
    ;;[0.0356 0.0356 0.0356] Finds What weapon player has equipped and plays different sound based on weapons
    ;;;[1 0 0] If and enemy hit player and another target sound error access none (disable enemies hitting each other or something else to fix this.
    (if _bsuccess
      (set `self.AttackRecieveSound` (`/Game/CombatFrameWork/Blueprints/Equipment/BP_BaseWeapon.Sound` (`/Game/CombatFrameWork/Blueprints/Components/BP_Combat.MainHandWeapon` (`/Game/ThirdPerson/Blueprints/BP_CombatCharacter.BP_Combat` _asbp_combat_character))))
      (else
        (set `self.AttackRecieveSound` (`/Game/CombatFrameWork/AI/BP_MasterEnemy.AttackSound` (cast `/Game/CombatFrameWork/AI/BP_MasterEnemy` _returnvalue :!pure true)))))
    (`self.Impact Effects` HitLocation)
    (`self.Hit Reaction` _returnvalue)
    (set `self.ArrowTag` (`self.ActorHasTag` DamageCauser "Arrow"))))

(event `Impact Effects`
  (params (Location :type "Vector Structure"))
  ;[0 0.9124 1] Find Sounds for different weapon types
  (`GameplayStatics.PlaySoundAtLocation` (`self.AttackRecieveSound`) Location (struct) 1.0 1.0 0.0 null null null null)
  (`GameplayStatics.SpawnEmitterAtLocation` "/Game/CombatFrameWork/MarketplaceAssests/Realistic_Starter_VFX_Pack_Vol2/Particles/Blood/P_Blood_Splat_Cone.P_Blood_Splat_Cone" Location))

(event `Hit Reaction`
  (params (Actor :type "Actor Object Reference"))
  (`GameplayStatics.PlayWorldCameraShake` "/Game/CombatFrameWork/Blueprints/CameraShake/BP_CameraShake.BP_CameraShake_C" (`self.K2_GetActorLocation`) (`self.Inner Radius`) (`self.Outer Radius`) (`self.Falloff`))
  (if (`self.CanBeStunned?`)
    (`/Game/CombatFrameWork/Blueprints/Components/BP_State.Set State` (`self.BP_State`) (struct :`TagName` "Player.State.Stunned")))
  (bind _returnvalue (`self.PlayAnimMontage` (`self.Get Hit React Animation` Actor)))
  (`KismetSystemLibrary.Delay` _returnvalue)
  (`/Game/CombatFrameWork/Blueprints/Components/BP_State.Clear State` (`self.BP_State`)))

(event `DeathEvents`
  (bind _healthbar (`self.Healthbar`))
  (`/Game/CombatFrameWork/Blueprints/Components/BP_State.Set State` (`self.BP_State`) (struct :`TagName` "Player.State.Death") :!label _label)
  (`/Engine/EditorBlueprintResources/StandardMacros.IsValid` _healthbar
    (:`Is Valid`
      (`ActorComponent.K2_DestroyComponent` _healthbar)
      (`/Game/CombatFrameWork/Blueprints/Components/BP_Collision.Turn Off Colliison` (`self.BP_Collision`))
      (`KismetSystemLibrary.Delay` 5.0)
      (`self.K2_DestroyActor`))))

(event `self.BP_Stats.Death`
  (bind _capsulecomponent (`self.CapsuleComponent`))
  (bind _mesh (`self.Mesh`))
  ;[0.9504 1 0] Add dissovler or emmitter on death. And maybe drops and exp
  (`BrainComponent.StopLogic` (`AIController.BrainComponent` (`AIBlueprintHelperLibrary.GetAIController` self)) "Death")
  (`self.StopAnimMontage` null)
  (`PrimitiveComponent.SetCollisionResponseToChannel` _capsulecomponent "ECC_Pawn" "ECR_Ignore")
  (`ActorComponent.K2_DestroyComponent` _capsulecomponent)
  (`PrimitiveComponent.SetCollisionProfileName` _mesh "Ragdoll" true)
  (`PrimitiveComponent.SetCollisionResponseToChannel` _mesh "ECC_Camera" "ECR_Ignore")
  (`PrimitiveComponent.SetSimulatePhysics` _mesh true)
  (goto _label))

(event `/Game/CombatFrameWork/Blueprints/Interfaces/BP_Targeting.OnTargeted`
  (params (`Targeted?` :type Boolean))
  (`SceneComponent.SetVisibility` (`self.LockOn Widget`) `Targeted?` false))

(event `/Game/CombatFrameWork/Blueprints/Interfaces/BP_Combat.Parried`
  (`/Game/CombatFrameWork/Blueprints/Components/BP_State.Set State` (`self.BP_State`) (struct :`TagName` "Player.State.Parried"))
  (`self.StopAnimMontage` null)
  (bind _returnvalue (`self.PlayAnimMontage` (`self.ParriedAnimation`)))
  (`KismetSystemLibrary.Delay` _returnvalue)
  (`/Game/CombatFrameWork/Blueprints/Components/BP_State.Clear State` (`self.BP_State`)))

(event `Sees Target`
  (params (Actor :type "Actor Object Reference")))

(event `/Game/CombatFrameWork/Blueprints/Interfaces/BP_Combat.StealthKilled`
  (`BrainComponent.StopLogic` (`AIController.BrainComponent` (`AIBlueprintHelperLibrary.GetAIController` self)) "")
  (`self.StopAnimMontage` null)
  (`self.PlayAnimMontage` "/Game/CombatFrameWork/Animations/StealthKill/A_Stealthkillvictem_Montage.A_Stealthkillvictem_Montage")
  (`self.DeathEvents`))

(event `/Game/CombatFrameWork/Blueprints/Interfaces/BP_Combat.Riposte`
  (`BrainComponent.StopLogic` (`AIController.BrainComponent` (`AIBlueprintHelperLibrary.GetAIController` self)) "RipostedKilled")
  (`self.StopAnimMontage` null)
  (`self.PlayAnimMontage` "/Game/CombatFrameWork/Animations/Riposte/A_RiposteVictem_Montage.A_RiposteVictem_Montage")
  (`self.DeathEvents`))

(fn `Calculate Damage`
  (returns (`Damage Amount` :type "Float (double-precision)"))
  (locals (NewLocalVar :type "Float (double-precision)" :default 0.0))
  (switch `/Game/CombatFrameWork/Blueprints/Enums/E_MontageAction` (`/Game/CombatFrameWork/Blueprints/Components/BP_State.Current Attack` (`self.BP_State`))
    (:`NewEnumerator2`
      (return (`self.BaseDamage`)))
    (:`NewEnumerator3`
      (return (* (`self.BaseDamage`) (`self.HeavyAttackMultiplier`))))
    (:`NewEnumerator4`
      (return (* (`self.BaseDamage`) (`self.Air Attack Multiplier`))))
    (:`NewEnumerator5`
      (return (* (`self.BaseDamage`) (`self.RunningAttackMultiplier`))))
    (:`NewEnumerator6`
      (return (* (`self.BaseDamage`) (`self.Special Attack Multi`))))))

(fn `CanBeRiposted?`
  (returns (`CanBeRiposted?` :type Boolean))
  (return (and (`/Game/CombatFrameWork/Blueprints/Components/BP_State.is Current State Equal To Any` (`self.BP_State`) (struct :`GameplayTags` (struct :`(TagName` "Player.State.Parried")))) (not (`/Game/CombatFrameWork/Blueprints/Components/BP_State.is Current State Equal To Any` (`self.BP_State`) (struct :`GameplayTags` (struct :`(TagName` "Player.State.Death"))))))))

(fn `CanBeStealthKilled`
  (returns (`CanBeStealthKilled?` :type Boolean))
  (return (and (`BlackboardComponent.GetValueAsBool` (`AIBlueprintHelperLibrary.GetBlackboard` (`self.GetController`)) "Stealth") (not (`/Game/CombatFrameWork/Blueprints/Components/BP_State.is Current State Equal To Any` (`self.BP_State`) (struct :`GameplayTags` (struct :`(TagName` "Player.State.Death"))))))))

(fn `CanBeTargeted`
  (returns (ReturnValue :type Boolean))
  (return (not (`/Game/CombatFrameWork/Blueprints/Components/BP_State.is Current State Equal To Any` (`self.BP_State`) (struct :`GameplayTags` (struct :`(TagName` "Player.State.Death")))))))

(fn `Create Health bar`
  (bind _aswb_stat_bar (cast `/Game/CombatFrameWork/Blueprints/Widgets/WB_StatBar` (`WidgetComponent.GetWidget` (`self.Healthbar`))))
  (bind _output_get (set `self.As WB Stat Bar` _aswb_stat_bar))
  (set `/Game/CombatFrameWork/Blueprints/Widgets/WB_StatBar.Stat` "NewEnumerator0" _output_get)
  (`/Game/CombatFrameWork/Blueprints/Widgets/WB_StatBar.Set Stat bar` _output_get (`self.BP_Stats`))
  (set `/Game/CombatFrameWork/Blueprints/Widgets/WB_StatBar.Fill Color And Opacity` (struct :`R` 1.0 :`B` 0.01736 :`A` 1.0) _output_get))

(fn `Get Hit React Animation`
  (params (Actor :type "Actor Object Reference"))
  (returns (AnimationMontage :type "AnimMontage Object Reference"))
  (locals (HitDIrection :type "/Game/CombatFrameWork/Blueprints/Enums/E_HitDirection Enum"))
  (bind (_returnvalue_roll _returnvalue_pitch _returnvalue_yaw) (`KismetMathLibrary.BreakRotator` (`KismetMathLibrary.NormalizedDeltaRotator` (`self.K2_GetActorRotation`) (`KismetMathLibrary.FindLookAtRotation` (`self.K2_GetActorLocation`) (`self.K2_GetActorLocation` Actor)))))
  (if (`KismetMathLibrary.InRange_FloatFloat` _returnvalue_yaw -45.0 45.0)
    (set `local.HitDIrection` "NewEnumerator0")
    (elif (`KismetMathLibrary.InRange_FloatFloat` _returnvalue_yaw -135.0 -45.0)
      (set `local.HitDIrection` "NewEnumerator3")
      (elif (or (`KismetMathLibrary.InRange_FloatFloat` _returnvalue_yaw 135.0 180.0) (`KismetMathLibrary.InRange_FloatFloat` _returnvalue_yaw -135.0 -180.0))
        (set `local.HitDIrection` "NewEnumerator1")
        (elif (`KismetMathLibrary.InRange_FloatFloat` _returnvalue_yaw 45.0 135.0)
          (set `local.HitDIrection` "NewEnumerator2")
          (else
            (set `local.HitDIrection` "NewEnumerator1"))))))
  (switch `/Game/CombatFrameWork/Blueprints/Enums/E_HitDirection` (`local.HitDIrection`)
    (:`NewEnumerator0`
      (return (`self.FrontHitReact`)))
    (:`NewEnumerator1`
      (return (`self.BackHitReact`)))
    (:`NewEnumerator2`
      (return (`self.LeftHitReact`)))
    (:`NewEnumerator3`
      (return (`self.RightHitReact`)))))

(fn `PerformAttack`
  (params (AttackType :type "/Game/CombatFrameWork/Blueprints/Enums/E_MontageAction Enum" :default "NewEnumerator0"))
  (returns (`Attack Duration` :type "Float (double-precision)"))
  (set `/Game/CombatFrameWork/Blueprints/Components/BP_State.Current Attack` AttackType (`self.BP_State`))
  (switch `/Game/CombatFrameWork/Blueprints/Enums/E_MontageAction` AttackType
    (:`NewEnumerator2`
      (`/Game/CombatFrameWork/Blueprints/Components/BP_Stats.Decrease Stamina` (`self.BP_Stats`) (`self.LightAttackStaminaCost`))
      (bind _returnvalue (`self.PlayAnimMontage` (`KismetArrayLibrary.Array_Random` (`self.lightAttacks`))))
      (return _returnvalue))
    (:`NewEnumerator3`
      (`/Game/CombatFrameWork/Blueprints/Components/BP_Stats.Decrease Stamina` (`self.BP_Stats`) (`self.HeavyAttackStaminaCost`))
      (bind _returnvalue_2 (`self.PlayAnimMontage` (`KismetArrayLibrary.Array_Random` (`self.HeavyAttacks`))))
      (return _returnvalue_2))
    (:`NewEnumerator4`
      (`/Game/CombatFrameWork/Blueprints/Components/BP_Stats.Decrease Stamina` (`self.BP_Stats`) (`self.AirAttackStaminaCost`))
      (bind _returnvalue_3 (`self.PlayAnimMontage` (`KismetArrayLibrary.Array_Random` (`self.AirAttack`))))
      (return _returnvalue_3))
    (:`NewEnumerator6`
      (`/Game/CombatFrameWork/Blueprints/Components/BP_Stats.Decrease Stamina` (`self.BP_Stats`) (`self.SpecialAttackStaminaCost`))
      (bind _returnvalue_4 (`self.PlayAnimMontage` (`KismetArrayLibrary.Array_Random` (`self.SpecialAttacks`))))
      (return _returnvalue_4))))

(fn `Toggle Health Bar`
  (params (Visibility :type Boolean))
  (bind _healthbar (`self.Healthbar`))
  (`/Engine/EditorBlueprintResources/StandardMacros.IsValid` _healthbar
    (:`Is Valid`
      (`SceneComponent.SetVisibility` _healthbar Visibility false))))

(fn `UserConstructionScript`)