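; Combat stats component that manages health, stamina, mana and defense for its owning actor.
; Spend, restore and damage functions update the values and broadcast UpdateStat for each change.
; Stamina and mana regenerate on looping timers, started through delayed gates that can be cancelled and stopped at max.
; Damage is scaled against defense, and zero health fires Death and sets the owner's BP_State to Death.
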(event `RefreshStamina`
  (params (StartStaminaRegeneration :type Boolean))
  ;[0.01938 0.01938 0.01938] Stamina
  (if StartStaminaRegeneration
    (`KismetSystemLibrary.K2_SetTimer` null "Regenerate Stamina" 0.1 true)
    (else
      (`KismetSystemLibrary.K2_ClearTimer` null "Regenerate Stamina"))))

(event `Handle Stamina Regeneration event`
  (params (`Start Refresh Stamina` :type Boolean) (Duration :type "Float (double-precision)"))
  ;[0.01938 0.01938 0.01938] Stamina
  (`self.Handle Stamina Regeneration` `Start Refresh Stamina` Duration))

(event `RefreshMana`
  (params (StartManaRegeneration :type Boolean))
  ;[0.01938 0.01938 0.01938] Mana
  (if StartManaRegeneration
    (`KismetSystemLibrary.K2_SetTimer` null "Regenerate Mana" 0.1 true)
    (else
      (`KismetSystemLibrary.K2_ClearTimer` null "Regenerate Mana"))))

(event `Handle Mana Regeration Event`
  (params (`Start Refresh Mana` :type Boolean) (Duration :type "Float (double-precision)"))
  ;[0.01938 0.01938 0.01938] Mana
  (`self.Handle Mana Regeneration` `Start Refresh Mana` Duration))

(fn `Check Player Has Enough Mana`
  (params (ManaCost :type "Float (double-precision)"))
  (returns (ReturnValue :type Boolean))
  (return (>= (`self.BaseMana`) ManaCost)))

(fn `Check Player Has Enough Stamina`
  (params (StaminaCost :type "Float (double-precision)"))
  (returns (ReturnValue :type Boolean))
  (return (>= (`self.BaseStamina`) StaminaCost)))

(fn `Decrease Mana`
  (params (ManaCost :type "Float (double-precision)"))
  (set `self.BaseMana` (`KismetMathLibrary.FClamp` (- (`self.BaseMana`) ManaCost) 0.0 (`self.MaxMana`)))
  (`self.UpdateStat` "NewEnumerator2"))

(fn `Decrease Stamina`
  (params (StaminaCost :type "Float (double-precision)"))
  (set `self.BaseStamina` (`KismetMathLibrary.FClamp` (- (`self.BaseStamina`) StaminaCost) 0.0 (`self.MaxStamina`)))
  (`self.UpdateStat` "NewEnumerator1"))

(fn `DecreaseDefense`
  (params (DefenseAmount :type "Float (double-precision)"))
  (set `self.DefenseStat` (- DefenseAmount (`self.DefenseStat`))))

(fn `HealPlayer`
  (params (HealAmount :type "Float (double-precision)"))
  (set `self.Base Health` (`KismetMathLibrary.FClamp` (+ HealAmount (`self.Base Health`)) 0.0 (`self.Max Health`)))
  (`self.UpdateStat` "NewEnumerator0"))

(fn `IncreaseDefense`
  (params (DefenseAmount :type "Float (double-precision)"))
  (set `self.DefenseStat` (+ DefenseAmount (`self.DefenseStat`))))

(fn `Regenerate Mana`
  ;[0.0356 0.0356 0.0356] EP 3-4
  (bind _output_get (set `self.BaseMana` (+ (`self.BaseMana`) (`self.RegenerateMana`))))
  (`self.UpdateStat` "NewEnumerator2")
  (if (>= _output_get (`self.MaxMana`))
    (`self.RefreshMana` false)))

(fn `Regenerate Stamina`
  ;[0.0356 0.0356 0.0356] EP 3-4
  (bind _output_get (set `self.BaseStamina` (+ (`self.BaseStamina`) (`self.StaminaRegenerate`))))
  (`self.UpdateStat` "NewEnumerator1")
  (if (>= _output_get (`self.MaxStamina`))
    (`self.RefreshStamina` false)))

(fn `RestorePlayerMana`
  (params (ManaRestoreAmount :type "Float (double-precision)"))
  (set `self.BaseMana` (`KismetMathLibrary.FClamp` (+ ManaRestoreAmount (`self.BaseMana`)) 0.0 (`self.MaxMana`)))
  (`self.UpdateStat` "NewEnumerator2"))

(fn `RestorePlayerStamina`
  (params (RestoreStaminaAmount :type "Float (double-precision)"))
  (set `self.BaseStamina` (`KismetMathLibrary.FClamp` (+ RestoreStaminaAmount (`self.BaseStamina`)) 0.0 (`self.MaxStamina`)))
  (`self.UpdateStat` "NewEnumerator1"))

(fn `Take Damage`
  (params (`Damage Amount` :type "Float (double-precision)"))
  (bind _returnvalue (`KismetMathLibrary.FClamp` `Damage Amount` 0.0 (* (`local.Damage Amount`) (/ (`local.Damage Amount`) (+ (`local.Damage Amount`) (`self.DefenseStat`))))))
  (`KismetSystemLibrary.PrintString` (`KismetStringLibrary.Conv_DoubleToString` _returnvalue))
  (bind _output_get (set `self.Base Health` (- (`self.Base Health`) _returnvalue)))
  (`self.UpdateStat` "NewEnumerator0")
  (if (<= _output_get 0.0)
    (`self.Death`)
    (`/Game/CombatFrameWork/Blueprints/Components/BP_State.Set State` (`Actor.GetComponentByClass` (`self.GetOwner`) "/Game/CombatFrameWork/Blueprints/Components/BP_State.BP_State_C") (struct :`TagName` "Player.State.Death"))))