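; Base weapon actor for melee combat that attaches to its owner, sets the combat animation mode, repositions any shield and deals point damage through a collision component.
; Damage, stamina and mana costs follow the current attack type from BP_State.
; An animation DataTable supplies action montages through a combo index that resets after a retriggerable delay, plus directional hit reactions and dodge rolls.
; A mana-based damage reduction branch is left disconnected.
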(event `self.ReceiveTick`
  (params (DeltaSeconds :type "Float (single-precision)"))
  (`parent.ReceiveTick` DeltaSeconds))

(event `AttackComboCounter`
  (`/Engine/EditorBlueprintResources/StandardMacros.IncrementInt` (`self.AnimationIndex`)
    (:`  `
      ;[1 1 1] Causes issues if duration is too low or high when reset animation is triggered. Mess with the reset in the animations as well to start and stop combos and walking nicely. Polish thing not super importent
      (`KismetSystemLibrary.RetriggerableDelay` 2.0)
      (set `self.AnimationIndex` 0 :!label _label))))

(event `Reset Animation Index`
  (goto _label))

(event `self.BP_Collision.Damage Actor`
  (params (`Hit Data` :type "HitResult Structure"))
  (bind _returnvalue (`self.GetOwner`))
  (`GameplayStatics.ApplyPointDamage` (`.HitActor` (`GameplayStatics.BreakHitResult` `Hit Data`)) (`self.Attack Damage`) (`self.GetActorForwardVector` _returnvalue) `Hit Data` (`self.GetInstigatorController` _returnvalue) self))

(fn `Activate Collision`
  (params (CollisionType :type "/Game/CombatFrameWork/Blueprints/Enums/E_CollisionType Enum" :default "NewEnumerator0"))
  (switch `/Game/CombatFrameWork/Blueprints/Enums/E_CollisionType` CollisionType
    (:`NewEnumerator0`
      (`/Game/CombatFrameWork/Blueprints/Components/BP_Collision.Turn On Collision` (`self.BP_Collision`)))))

(fn `Attack Damage`
  (returns (BaseDamage :type "Float (double-precision)"))
  (switch `/Game/CombatFrameWork/Blueprints/Enums/E_MontageAction` (`/Game/CombatFrameWork/Blueprints/Components/BP_State.Current Attack` (`self.GetComponentByClass` (`self.GetOwner`) "/Game/CombatFrameWork/Blueprints/Components/BP_State.BP_State_C"))
    (:`NewEnumerator2`
      (return (`self.BaseDamage`)))
    (:`NewEnumerator3`
      (return (* (`self.BaseDamage`) (`self.Heavy Attack Multiplier`))))
    (:`NewEnumerator4`
      (return (* (`self.BaseDamage`) (`self.Air Attack Multiplier`))))
    (:`NewEnumerator5`
      (return (* (`self.BaseDamage`) (`self.Running Attack Multiplier`))))
    (:`NewEnumerator6`
      (return (* (`self.BaseDamage`) (`self.Charged Attack Multiplier`))))))

(fn `Deactivate Collision`
  (`/Game/CombatFrameWork/Blueprints/Components/BP_Collision.Turn Off Colliison` (`self.BP_Collision`)))

(fn `Equip Item`
  (locals (LocalShield :type "/Game/CombatFrameWork/Blueprints/Equipment/BP_BaseOffhand Object Reference"))
  (bind _localshield (`local.LocalShield`))
  (bind _localshield_2 (`local.LocalShield`))
  ;[0.0356 0.0356 0.0356] Weapon Ep 1 Equipping to sockets
  (bind _output_get (set `self.Combat Component Ref` (`self.GetComponentByClass` (`self.GetOwner`) "/Game/CombatFrameWork/Blueprints/Components/BP_Combat.BP_Combat_C")))
  (`/Game/CombatFrameWork/Blueprints/Components/BP_Combat.SetMainHand` _output_get self)
  (`self.Attach To Player` (select `bool` (`/Game/CombatFrameWork/Blueprints/Components/BP_Combat.CombatEnabled?` (`self.Combat Component Ref`)) :`false` (`self.UnequippedSocket`) :`true` (`self.EquippedSocket`)))
  ;[0.01938 0.01938 0.01938] Ep.1 Collision System
  (`/Game/CombatFrameWork/Blueprints/Components/BP_Collision.Set Weapon` (`self.BP_Collision`) (`self.StaticMesh`))
  ;;[0.01938 0.01938 0.01938] Updates Combat type to use different locomotion animations based on weapon // Ep3 Weapon types
  (message `/Game/CombatFrameWork/Blueprints/Interfaces/BP_Animation.UpdateCombatMode` (`SkeletalMeshComponent.GetAnimInstance` (`Character.Mesh` (cast `Character` (`self.GetOwner`) :!pure true))) (`self.CombatType`))
  (`KismetArrayLibrary.Array_Add` (`/Game/CombatFrameWork/Blueprints/Components/BP_Collision.Actors to Ignore` (`self.BP_Collision`)) (`self.GetOwner`))
  ;[0.01938 0.01938 0.01938] Shield Equip socket based off what weapon player is weilding
  (bind _output_get_2 (set `local.LocalShield` (`/Game/CombatFrameWork/Blueprints/Components/BP_Combat.MainOffhand` (`self.Combat Component Ref`))))
  (`/Engine/EditorBlueprintResources/StandardMacros.IsValid` _output_get_2
    (:`Is Valid`
      (switch `/Game/CombatFrameWork/Blueprints/Enums/E_CombatType` (`self.CombatType`)
        (:`NewEnumerator0`
          (`self.Attach To Player` _localshield_2 (`/Game/CombatFrameWork/Blueprints/Equipment/BP_BaseOffhand.UnequippedSocket` _localshield_2) :!label _label))
        (:`NewEnumerator1`
          (`self.Attach To Player` _localshield (select `bool` (`/Game/CombatFrameWork/Blueprints/Components/BP_Combat.CombatEnabled?` (`self.Combat Component Ref`)) :`false` (`/Game/CombatFrameWork/Blueprints/Equipment/BP_BaseOffhand.UnequippedSocket` _localshield) :`true` (`/Game/CombatFrameWork/Blueprints/Equipment/BP_BaseOffhand.EquippedSocket` _localshield))))
        (:`NewEnumerator2`
          (goto _label))
        (:`NewEnumerator3`
          (goto _label))
        (:`NewEnumerator4`
          (goto _label))))))

(fn `Get Hit Reaction`
  (params (Action :type "/Game/CombatFrameWork/Blueprints/Enums/E_MontageAction Enum" :default "NewEnumerator0") (Actor :type "Actor Object Reference"))
  (returns (Output :type "AnimMontage Object Reference"))
  (bind _returnvalue (`self.GetOwner`))
  (bind (_returnvalue_roll _returnvalue_pitch _returnvalue_yaw) (`KismetMathLibrary.BreakRotator` (`KismetMathLibrary.NormalizedDeltaRotator` (`self.K2_GetActorRotation` _returnvalue) (`KismetMathLibrary.FindLookAtRotation` (`self.K2_GetActorLocation` _returnvalue) (`self.K2_GetActorLocation` Actor)))))
  ;[0.0356 0.0356 0.0356] Player getting attack hit reaction ep. 5 enemy ai system
  (bind _returnvalue_2 (`|GetDataTableRow` (`self.AnimationDataTable`) (`KismetStringLibrary.Conv_StringToName` (`|GetEnumeratorNameAsString` Action)))
    (:`then`
      (if (`KismetMathLibrary.InRange_FloatFloat` _returnvalue_yaw -45.0 45.0)
        (bind ((`Animation_6_9079765444AAD99A6A82E0B8B6762871` _animation)) (break `/Game/CombatFrameWork/Blueprints/Structures/S_MontageAction` _returnvalue_2))
        (return (`|GetArrayItem` _animation))
        (elif (`KismetMathLibrary.InRange_FloatFloat` _returnvalue_yaw -135.0 -45.0)
          (return (`|GetArrayItem` _animation 1))
          (elif (or (`KismetMathLibrary.InRange_FloatFloat` _returnvalue_yaw 135.0 180.0) (`KismetMathLibrary.InRange_FloatFloat` _returnvalue_yaw -135.0 -180.0))
            (return (`|GetArrayItem` _animation 2))
            (elif (`KismetMathLibrary.InRange_FloatFloat` _returnvalue_yaw 45.0 135.0)
              (return (`|GetArrayItem` _animation 3))
              (else
                (return (`|GetArrayItem` _animation 2))))))))))

(fn `Get Mana Cost For Attack`
  (returns (`Mana Cost` :type "Float (double-precision)"))
  (switch `/Game/CombatFrameWork/Blueprints/Enums/E_MontageAction` (`/Game/CombatFrameWork/Blueprints/Components/BP_State.Current Attack` (`self.GetComponentByClass` (`self.GetOwner`) "/Game/CombatFrameWork/Blueprints/Components/BP_State.BP_State_C"))
    (:`NewEnumerator2`
      (return (`self.Light Attack Mana Cost`)))
    (:`NewEnumerator3`
      (return (`self.Heavy Attack Mana Cost`)))
    (:`NewEnumerator4`
      (return (`self.Air Attack Mana Cost`)))
    (:`NewEnumerator5`
      (return (`self.Running Attack Mana Cost`)))
    (:`NewEnumerator6`
      (return (`self.Charged Attack Mana Cost`)))))

(fn `Get Montage For Action`
  (params (Action :type "/Game/CombatFrameWork/Blueprints/Enums/E_MontageAction Enum" :default "NewEnumerator0"))
  (returns (Output :type "AnimMontage Object Reference"))
  ;[0.0356 0.0356 0.0356] EP 5 Animation montage for equips // EP.1 attacking we the last half of this function and replaced the index with the animation index.
  (bind _returnvalue (`|GetDataTableRow` (`self.AnimationDataTable`) (`KismetStringLibrary.Conv_StringToName` (`|GetEnumeratorNameAsString` Action)))
    (:`then`
      (bind ((`Animation_6_9079765444AAD99A6A82E0B8B6762871` _animation)) (break `/Game/CombatFrameWork/Blueprints/Structures/S_MontageAction` _returnvalue))
      (if (>= (`self.AnimationIndex`) (- (`KismetArrayLibrary.Array_Length` _animation) 1))
        (`self.Reset Animation Index`)
        (return (`|GetArrayItem` _animation (`KismetArrayLibrary.Array_LastIndex` _animation)))
        (else
          (`self.AttackComboCounter`)
          (return (`|GetArrayItem` _animation (- (`self.AnimationIndex`) 1))))))))

(fn `Get Stamina Cost For Attack`
  (returns (`Stamina Cost` :type "Float (double-precision)"))
  (switch `/Game/CombatFrameWork/Blueprints/Enums/E_MontageAction` (`/Game/CombatFrameWork/Blueprints/Components/BP_State.Current Attack` (`self.GetComponentByClass` (`self.GetOwner`) "/Game/CombatFrameWork/Blueprints/Components/BP_State.BP_State_C"))
    (:`NewEnumerator2`
      (return (`self.Light Attack Cost`)))
    (:`NewEnumerator3`
      (return (`self.Heavy Attack Cost`)))
    (:`NewEnumerator4`
      (return (`self.Air Attack Cost`)))
    (:`NewEnumerator5`
      (return (`self.Running Attack Cost`)))
    (:`NewEnumerator6`
      (return (`self.Charged Attack Cost `)))))

(fn `GetDodgeRollAnimation`
  (params (Action :type "/Game/CombatFrameWork/Blueprints/Enums/E_MontageAction Enum" :default "NewEnumerator0") (DodgeRollIndex :type Integer))
  (returns (Output :type "AnimMontage Object Reference"))
  (bind _returnvalue (`|GetDataTableRow` (`self.AnimationDataTable`) (`KismetStringLibrary.Conv_StringToName` (`|GetEnumeratorNameAsString` Action)))
    (:`then`
      (return (`|GetArrayItem` (`.Animation_6_9079765444AAD99A6A82E0B8B6762871` (break `/Game/CombatFrameWork/Blueprints/Structures/S_MontageAction` _returnvalue)) DodgeRollIndex)))))

(fn `UserConstructionScript`
  (`parent.UserConstructionScript`)
  (`StaticMeshComponent.SetStaticMesh` (`self.StaticMesh`) (`self.EquipmentMesh`)))