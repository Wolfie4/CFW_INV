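; Base Blueprint for dual-sword equipment, extending a parent weapon class with a second blade that uses the same equipment mesh.
; Attaching to the player also snaps the second mesh to its own equipped or unequipped socket on the Character, based on combat state.
; A second collision component traces that mesh, ignores the owner, and toggles alongside the parent's collision, which always receives a fixed collision type.
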(fn `Activate Collision`
  (params (CollisionType :type "/Game/CombatFrameWork/Blueprints/Enums/E_CollisionType Enum" :default "NewEnumerator0"))
  (`parent.Activate Collision` "NewEnumerator0")
  (`/Game/CombatFrameWork/Blueprints/Components/BP_Collision.Turn On Collision` (`self.BP_Collision1`)))

(fn `Attach Second Weapon`
  (params (Socket :type Name))
  (`SceneComponent.K2_AttachToComponent` (`self.StaticMesh1`) (`Character.Mesh` (cast `Character` (`self.GetOwner`) :!pure true)) Socket "SnapToTarget" "SnapToTarget" "SnapToTarget" true))

(fn `Attach To Player`
  (params (SocketName :type Name))
  (`parent.Attach To Player` SocketName)
  (`self.Attach Second Weapon` (select `bool` (`/Game/CombatFrameWork/Blueprints/Components/BP_Combat.CombatEnabled?` (`self.Combat Component Ref`)) :`false` (`self.SecondUnequippedSocket`) :`true` (`self.SecondEquippedSocket`))))

(fn `Deactivate Collision`
  (`parent.Deactivate Collision`)
  (`/Game/CombatFrameWork/Blueprints/Components/BP_Collision.Turn Off Colliison` (`self.BP_Collision1`)))

(fn `Equip Item`
  (`parent.Equip Item`)
  (`/Game/CombatFrameWork/Blueprints/Components/BP_Collision.Set Weapon` (`self.BP_Collision1`) (`self.StaticMesh1`))
  (`KismetArrayLibrary.Array_Add` (`/Game/CombatFrameWork/Blueprints/Components/BP_Collision.Actors to Ignore` (`self.BP_Collision1`)) (`self.GetOwner`)))

(fn `UserConstructionScript`
  (`parent.UserConstructionScript`)
  (`StaticMeshComponent.SetStaticMesh` (`self.StaticMesh1`) (`self.EquipmentMesh`)))