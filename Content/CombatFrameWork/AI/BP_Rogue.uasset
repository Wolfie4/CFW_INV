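; BP_Rogue is an AI enemy in the combat framework that deals melee damage with a JadeSword.
; On BeginPlay it runs parent setup and assigns the sword to its collision component, which activation events switch on for Main Weapon attacks and off afterward.
; Collision hits apply point damage only to the player character, using a calculated amount and BP_DamageType.
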(event `self.ReceiveBeginPlay`
  (`parent.ReceiveBeginPlay`)
  (`/Game/CombatFrameWork/Blueprints/Components/BP_Collision.Set Weapon` (`self.BP_Collision1`) (`self.JadeSword`)))

(event `self.BP_Collision1.Damage Actor`
  (params (`Hit Data` :type "HitResult Structure"))
  (bind (_bblockinghit _binitialoverlap _time _distance _location _impactpoint _normal _impactnormal _physmat _hitactor) (`GameplayStatics.BreakHitResult` `Hit Data`))
  (bind _returnvalue (`self.GetOwner`))
  ;[1 1 1] Enemy can only damage the player
  (if (== _hitactor (`GameplayStatics.GetPlayerCharacter` 0))
    (`GameplayStatics.ApplyPointDamage` _hitactor (`self.Calculate Damage`) (`self.GetActorForwardVector` _returnvalue) `Hit Data` (`self.GetInstigatorController` _returnvalue) null "/Game/CombatFrameWork/Blueprints/Damage/BP_DamageType.BP_DamageType_C")))

(event `self.ActivateCollision`
  (params (CollisionType :type "/Game/CombatFrameWork/Blueprints/Enums/E_CollisionType Enum" :default "NewEnumerator0"))
  (switch `/Game/CombatFrameWork/Blueprints/Enums/E_CollisionType` CollisionType
    (:`NewEnumerator0`
      (`/Game/CombatFrameWork/Blueprints/Components/BP_Collision.Turn On Collision` (`self.BP_Collision1`)))))

(event `self.DeactivateCollision`
  (`/Game/CombatFrameWork/Blueprints/Components/BP_Collision.Turn Off Colliison` (`self.BP_Collision1`)))

(fn `UserConstructionScript`
  (`parent.UserConstructionScript`))