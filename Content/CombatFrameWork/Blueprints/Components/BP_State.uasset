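; BP_State is a combat framework component that tracks its owner's current state, current attack and whether movement input is allowed.
; Helper functions set or clear the state gameplay tag and test it for an exact match against a tag container.
; MovementInputHandler either disables movement input immediately, or waits on a retriggerable delay before re-enabling it and clearing the state.
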(event `Movement Input Handler`
  (params (Duration :type "Float (double-precision)") (`Disable Input` :type Boolean))
  ;[0.01938 0.01938 0.01938] State System ep7
  (if `Disable Input`
    (set `self.Movement Input` false)
    (else
      (`KismetSystemLibrary.RetriggerableDelay` Duration)
      (set `self.Movement Input` true)
      (`self.Clear State`))))

(fn `Clear State`
  (set `self.Current State` (struct)))

(fn `is Current State Equal To Any`
  (params (`State To Check` :type "GameplayTagContainer Structure"))
  (returns (ReturnValue :type Boolean))
  (return (`BlueprintGameplayTagLibrary.HasTag` `State To Check` (`self.Current State`) true)))

(fn `Set Attack`
  (params (`Current Attack` :type "/Game/CombatFrameWork/Blueprints/Enums/E_MontageAction Enum" :default "NewEnumerator0"))
  (set `self.Current Attack` `Current Attack`))

(fn `Set State`
  (params (`New State` :type "GameplayTag Structure"))
  (set `self.Current State` `New State`))