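; BP_Fists is the unarmed weapon in the combat framework, using two collision components, one per fist.
; Equipping registers it as main hand on the owner's BP_Combat, enables combat, updates the anim instance's combat type and toggles equipment.
; Both collisions use the character mesh as their weapon and ignore the owner.
; Activation switches on one fist by collision type, while deactivation extends the parent's to turn off the second.
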(fn `Activate Collision`
  (params (CollisionType :type "/Game/CombatFrameWork/Blueprints/Enums/E_CollisionType Enum" :default "NewEnumerator0"))
  (switch `/Game/CombatFrameWork/Blueprints/Enums/E_CollisionType` CollisionType
    (:`NewEnumerator0`
      (`/Game/CombatFrameWork/Blueprints/Components/BP_Collision.Turn On Collision` (`self.BP_Collision`)))
    (:`NewEnumerator2`
      (`/Game/CombatFrameWork/Blueprints/Components/BP_Collision.Turn On Collision` (`self.BP_Collision1`)))))

(fn `Deactivate Collision`
  (`parent.Deactivate Collision`)
  (`/Game/CombatFrameWork/Blueprints/Components/BP_Collision.Turn Off Colliison` (`self.BP_Collision1`)))

(fn `Equip Item`
  (bind _bp_collision1 (`self.BP_Collision1`))
  (bind _output_get (set `self.Combat Component Ref` (`self.GetComponentByClass` (`self.GetOwner`) "/Game/CombatFrameWork/Blueprints/Components/BP_Combat.BP_Combat_C")))
  (`/Game/CombatFrameWork/Blueprints/Components/BP_Combat.SetMainHand` _output_get self)
  (`/Game/CombatFrameWork/Blueprints/Components/BP_Collision.Set Weapon` (`self.BP_Collision`) (`Character.Mesh` (cast `Character` (`self.GetOwner`) :!pure true)))
  (set `/Game/CombatFrameWork/Blueprints/Components/BP_Combat.CombatEnabled?` true _output_get)
  (message `/Game/CombatFrameWork/Blueprints/Interfaces/BP_Animation.UpdateCombatMode` (`SkeletalMeshComponent.GetAnimInstance` (`Character.Mesh` (cast `Character` (`self.GetOwner`) :!pure true))) (`self.CombatType`))
  (`/Game/CombatFrameWork/Blueprints/Components/BP_Combat.ToggleEquipment` (`self.Combat Component Ref`) true)
  (`KismetArrayLibrary.Array_Add` (`/Game/CombatFrameWork/Blueprints/Components/BP_Collision.Actors to Ignore` (`self.BP_Collision`)) (`self.GetOwner`))
  (`/Game/CombatFrameWork/Blueprints/Components/BP_Collision.Set Weapon` _bp_collision1 (`Character.Mesh` (cast `Character` (`self.GetOwner`) :!pure true)))
  (`KismetArrayLibrary.Array_Add` (`/Game/CombatFrameWork/Blueprints/Components/BP_Collision.Actors to Ignore` _bp_collision1) (`self.GetOwner`)))

(fn `UserConstructionScript`
  (`parent.UserConstructionScript`))