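; Base shield equipment for the combat framework, attached to its owner on a socket that suits the current weapon and combat state.
; The construction script applies the configured equipment mesh.
; Equipping registers the shield with the owner's BP_Combat component, then, if a main weapon exists, picks a socket from its combat type.
; Only Sword and Shield with combat enabled uses the equipped socket; other cases use the unequipped one.
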(fn `Equip Item`
  (bind _mainweapon (`/Game/CombatFrameWork/Blueprints/Components/BP_Combat.MainWeapon` (`self.Combat Component Ref`)))
  (bind _output_get (set `self.Combat Component Ref` (`self.GetComponentByClass` (`self.GetOwner`) "/Game/CombatFrameWork/Blueprints/Components/BP_Combat.BP_Combat_C")))
  (`/Game/CombatFrameWork/Blueprints/Components/BP_Combat.Set Shield` _output_get self)
  (`/Engine/EditorBlueprintResources/StandardMacros.IsValid` _mainweapon
    (:`Is Valid`
      (switch `/Game/CombatFrameWork/Blueprints/Enums/E_CombatType` (`/Game/CombatFrameWork/Blueprints/Equipment/BP_BaseWeapon.CombatType` _mainweapon)
        (:`NewEnumerator0`
          (`self.Attach To Player` (`self.UnequippedSocket`) :!label _label))
        (:`NewEnumerator1`
          (`self.Attach To Player` (select `bool` (`/Game/CombatFrameWork/Blueprints/Components/BP_Combat.CombatEnabled?` (`self.Combat Component Ref`)) :`false` (`self.UnequippedSocket`) :`true` (`self.EquippedSocket`))))
        (:`NewEnumerator2`
          (goto _label))
        (:`NewEnumerator3`
          (goto _label))
        (:`NewEnumerator4`
          (goto _label))))))

(fn `UserConstructionScript`
  (`StaticMeshComponent.SetStaticMesh` (`self.StaticMesh`) (`self.EquipmentMesh`)))