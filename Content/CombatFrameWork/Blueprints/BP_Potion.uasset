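; BP_Potion is the potion actor whose static mesh reflects the item equipped in the player's consumable slot.
; Change Potion Mesh reads consumable slot 1 from the passed equipment sheet, looks up that row in DataTable_Item and applies its mesh, printing a debug string when the reference is invalid.
; Empty Glass swaps one material slot to plain glass.
; An author comment notes the mesh change fails on a null equipment sheet access.
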(event `self.ReceiveBeginPlay`)

(fn `Change Potion Mesh`
  (params (`Equipment sheet ref` :type "/Game/Inventory/Blueprints/BP_Inventory Object Reference"))
  ;[1 0 0] gets the item in the consumable slot, gets it mesh and changes the mesh to match whatever potion is in there. // Fails because accessing none trying to read the equipment sheet
  (`/Engine/EditorBlueprintResources/StandardMacros.IsValid` `Equipment sheet ref`
    (:`Is Valid`
      (bind _returnvalue (`|GetDataTableRow` "/Game/Inventory/DataTable/DataTable_Item.DataTable_Item" (`.RowName` (break `DataTableRowHandle` (`.DataTable_6_775A83664656B010A5EE4FBC86628E06` (break `/Game/Inventory/Structures/S_ItemMaster` (`/Game/Inventory/WidgetBlueprints/WB_EquipmentSlot.Item` (`/Game/Inventory/WidgetBlueprints/WB_EquipmentSheet.WB_ConsumableSlot1` (`/Game/Inventory/Blueprints/BP_Inventory.EquipmentSheet` `Equipment sheet ref`))))))))
        (:`then`
          (`StaticMeshComponent.SetStaticMesh` (`self.Potion`) (`.Mesh_18_B5102D874A8CB20FF58A70AEFA7CBAB8` (break `/Game/Inventory/Structures/S_Item` _returnvalue)))
          (return))))
    (:`Is Not Valid`
      (`KismetSystemLibrary.PrintString` "sadge"))))

(fn `Empty Glass`
  (`PrimitiveComponent.SetMaterial` (`self.Potion`) 2 "/Game/CombatFrameWork/Meshes/Misc/Potion/M_Glass.M_Glass"))

(fn `UserConstructionScript`)