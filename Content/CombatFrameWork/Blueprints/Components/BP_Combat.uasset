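; BP_Combat is a combat component that tracks the equipped main-hand weapon and offhand item, such as a shield.
; SetMainHand and SetOffhand destroy any valid actor already in that slot, store the new one, then trigger a UI update through CallUpdateUI.
; RemoveOffhand clears the offhand reference and updates the UI without destroying the actor.
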(fn `RemoveOffhand`
  (set `self.MainOffhand` null)
  (`self.UpdateUI`))

(fn `SetMainHand`
  (params (`New Weapon` :type "/Game/CombatFrameWork/Blueprints/Equipment/BP_BaseWeapon Object Reference"))
  ;[0.0356 0.0356 0.0356] Weapon Swap if on is equipped
  (`|ExecutionSequence`
    (:`then_0`
      (`/Engine/EditorBlueprintResources/StandardMacros.IsValid` (`self.MainWeapon`)
        (:`Is Valid`
          (`Actor.K2_DestroyActor` (`self.MainWeapon`)))))
    (:`then_1`
      (set `self.MainWeapon` `New Weapon`)
      (`self.UpdateUI`))))

(fn `SetOffhand`
  (params (Shield :type "/Game/CombatFrameWork/Blueprints/Equipment/BP_Offhand Object Reference"))
  ;[0.0356 0.0356 0.0356] offhand Swap if on is equipped
  (`|ExecutionSequence`
    (:`then_0`
      (`/Engine/EditorBlueprintResources/StandardMacros.IsValid` (`self.MainOffhand`)
        (:`Is Valid`
          (`Actor.K2_DestroyActor` (`self.MainOffhand`)))))
    (:`then_1`
      (set `self.MainOffhand` Shield)
      (`self.UpdateUI`))))