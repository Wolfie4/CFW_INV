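; BP_Item is a world pickup actor that the player can add to an inventory.
; The construction script sets its mesh from a data table row in ItemData.
; A sphere overlap with the player toggles an outline overlay material and an interaction widget.
; Interact adds the item to the passed inventory, refreshes list and weight, then destroys the actor, or shows an inventory-full widget on failure.
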(event `self.Sphere.OnComponentBeginOverlap`
  (params (OverlappedComponent :type "PrimitiveComponent Object Reference") (OtherActor :type "Actor Object Reference") (OtherComp :type "PrimitiveComponent Object Reference") (OtherBodyIndex :type Integer) (bFromSweep :type Boolean) (SweepResult :type "HitResult Structure (by ref)"))
  (if (== OtherActor (`GameplayStatics.GetPlayerCharacter` 0))
    (`MeshComponent.SetOverlayMaterial` (`self.Item`) "/Game/Inventory/Materials/M_Outline_InstTest.M_Outline_InstTest")
    (`SceneComponent.SetVisibility` (`self.W_Interact`) true false)))

(event `self.Sphere.OnComponentEndOverlap`
  (params (OverlappedComponent :type "PrimitiveComponent Object Reference") (OtherActor :type "Actor Object Reference") (OtherComp :type "PrimitiveComponent Object Reference") (OtherBodyIndex :type Integer))
  (if (== OtherActor (`GameplayStatics.GetPlayerCharacter` 0))
    (`MeshComponent.SetOverlayMaterial` (`self.Item`) null)
    (`SceneComponent.SetVisibility` (`self.W_Interact`) false false)))

(event `/Game/CombatFrameWork/Blueprints/Interfaces/BP_Interact.Interact`
  (params (Actor :type "Actor Object Reference") (Inventory :type "/Game/Inventory/Blueprints/BP_Inventory Object Reference"))
  (bind _inventory (`/Game/Inventory/Blueprints/BP_Inventory.Inventory` Inventory))
  (bind _addeditemtoinventory (`/Game/Inventory/Blueprints/BP_Inventory.AddItemToInventory` Inventory (`self.ItemData`)))
  (if _addeditemtoinventory
    (`/Game/Inventory/WidgetBlueprints/WB_ItemSlotInventory.LoadInventory` (`/Game/Inventory/WidgetBlueprints/WB_Inventory.WB_ItemInventory` _inventory) Inventory)
    (`/Game/Inventory/WidgetBlueprints/WB_Inventory.UpdateWeight` _inventory)
    (`self.K2_DestroyActor`)
    (else
      (bind _inventoryfull (`self.InventoryFull`)
        (:`then`
          (`UserWidget.AddToViewport` _inventoryfull 0)
          (`/Game/Inventory/WidgetBlueprints/WB_InventroyFull.Play animation event` _inventoryfull))
        (:`else`
          (bind _returnvalue (`|CreateWidget` "/Game/Inventory/WidgetBlueprints/WB_InventroyFull.WB_InventroyFull_C"))
          (bind _output_get (set `self.InventoryFull` _returnvalue))
          (`UserWidget.AddToViewport` _output_get 0))))))

(fn `UserConstructionScript`
  (bind (_datatable _rowname) (break `DataTableRowHandle` (`.DataTable_6_775A83664656B010A5EE4FBC86628E06` (break `/Game/Inventory/Structures/S_ItemMaster` (`self.ItemData`)))))
  (bind _returnvalue (`|GetDataTableRow` _datatable _rowname)
    (:`then`
      (`StaticMeshComponent.SetStaticMesh` (`self.Item`) (`.Mesh_18_B5102D874A8CB20FF58A70AEFA7CBAB8` (break `/Game/Inventory/Structures/S_Item` _returnvalue))))))