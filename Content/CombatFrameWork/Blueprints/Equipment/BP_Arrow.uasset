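; BP_Arrow is a projectile arrow actor in the combat framework's equipment, launched through its FireArrow event.
; FireArrow adds a ProjectileMovementComponent at runtime, setting its velocity from the passed vector scaled by ArrowStrength and applying the configured gravity scale.
; It then attaches a Niagara trail effect to the Arrow component and stores references to both the movement component and the effect.
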(event `FireArrow`
  (params (Velocity :type "Vector Structure"))
  (bind _returnvalue (`AddComponent|NODE_AddProjectileMovementComponent-0`))
  (bind _output_get (set `self.ProjectileRef` _returnvalue))
  (set `MovementComponent.Velocity` (* Velocity (`self.ArrowStrength`)) _output_get)
  (set `ProjectileMovementComponent.ProjectileGravityScale` (`self.Projectile Gravity Scale`) _output_get)
  (bind _returnvalue_2 (`NiagaraFunctionLibrary.SpawnSystemAttached` (`self.ArrowTrail_NS`) (`self.Arrow`) "None" (0.0 0.0 0.0) (struct) "SnapToTarget"))
  (set `self.SystemRef` _returnvalue_2))

(fn `UserConstructionScript`)