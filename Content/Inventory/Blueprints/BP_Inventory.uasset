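; Player inventory component holding gear, consumable and ammo slot arrays, with input-toggled inventory and equipment sheet widgets.
; Sphere-trace interaction passes it to BP_Interact actors, while AddItemToInventory fills empty gear slots or stacks consumables by DataTable stack size, trying equipped slot 1 first.
; Consuming from that slot restores health through BP_Stats.
; BP_Save persists gear, consumables and equipped items, loaded at BeginPlay and saved or deleted by input.
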(event `self.ReceiveBeginPlay`
  (bind _returnvalue (`GameplayStatics.GetPlayerController` 0))
  ;[0.1797 1 0] Adds Input actions for inventory. Change to keybinds later i believe
  (`/Engine/EditorBlueprintResources/StandardMacros.IsValid` _returnvalue
    (:`Is Valid`
      (`EnhancedInputSubsystemInterface.AddMappingContext` (pcsubsystem `EnhancedInputLocalPlayerSubsystem` _returnvalue) "/Game/Inventory/Input/IMC_Inventory.IMC_Inventory" 0 (struct))
      (bind _returnvalue_2 (`|CreateWidget` "/Game/Inventory/WidgetBlueprints/WB_Inventory.WB_Inventory_C"))
      (bind _output_get (set `self.Inventory` _returnvalue_2))
      ;[1 1 1] Stack Sizes
      (`KismetArrayLibrary.Array_Resize` (`self.GearSlots`) (`self.GearSlotSize`))
      (`KismetArrayLibrary.Array_Resize` (`self.Consumable_Slots`) (`self.ConsumableSlotSize`))
      (`KismetArrayLibrary.Array_Resize` (`self.AmmoSlots`) (`self.AmmoSize`))
      ;[0.01938 0.01938 0.01938] Save Game
      (bind _returnvalue_3 (`GameplayStatics.DoesSaveGameExist` "inventory"))
      (if _returnvalue_3
        (bind _returnvalue_4 (`GameplayStatics.LoadGameFromSlot` "inventory"))
        (bind _asbp_save (cast `/Game/Inventory/Blueprints/BP_Save` _returnvalue_4))
        (bind _output_get_2 (set `self.Save Game` _asbp_save))
        (set `self.GearSlots` (`/Game/Inventory/Blueprints/BP_Save.Gear` _output_get_2))
        (set `self.Consumable_Slots` (`/Game/Inventory/Blueprints/BP_Save.Consumables` _output_get_2))
        (`self.LoadEquippedItems`))
      ;[1 1 1] refresh inventory
      (`/Game/Inventory/WidgetBlueprints/WB_ItemSlotInventory.LoadInventory` (`/Game/Inventory/WidgetBlueprints/WB_Inventory.WB_ItemInventory` _output_get) self)
      ;[1 1 1] May need to add load inventory or something
      (bind _returnvalue_5 (`|CreateWidget` "/Game/Inventory/WidgetBlueprints/WB_EquipmentSheet.WB_EquipmentSheet_C"))
      (set `self.EquipmentSheet` _returnvalue_5))))

(event `EnhancedInput|/Game/Inventory/Input/IA_Interact`
  (params (ActionValue :type Boolean) (ElapsedSeconds :type "Float (double-precision)") (TriggeredSeconds :type "Float (double-precision)") (InputAction :type "InputAction Object Reference" :default "/Game/Inventory/Input/IA_Interact.IA_Interact"))
  (:`Started`
    (`self.Interact`)))

(event `EnhancedInput|/Game/Inventory/Input/IA_Inventory`
  (params (ActionValue :type Boolean) (ElapsedSeconds :type "Float (double-precision)") (TriggeredSeconds :type "Float (double-precision)") (InputAction :type "InputAction Object Reference" :default "/Game/Inventory/Input/IA_Inventory.IA_Inventory"))
  (bind _returnvalue (`GameplayStatics.GetPlayerController` 0))
  (bind _returnvalue_2 (`GameplayStatics.GetPlayerController` 0))
  ;[0.008023 0.008023 0.008023] Loads Inventory Sheet Widget
  (:`Started`
    (if (`Widget.IsVisible` (`self.Inventory`))
      ;;[0.9647 1 0] Find a more eligent way to check if a ui window is open. Especially when crafting windows or something is added
      (if (not (`Widget.IsVisible` (`self.EquipmentSheet`)))
        (set `PlayerController.bShowMouseCursor` false _returnvalue_2)
        (`WidgetBlueprintLibrary.SetInputMode_GameOnly` _returnvalue_2))
      (`Widget.RemoveFromParent` (`self.Inventory`))
      (else
        (set `PlayerController.bShowMouseCursor` true _returnvalue)
        (`WidgetBlueprintLibrary.SetInputMode_GameAndUIEx` _returnvalue (`self.Inventory`))
        (`UserWidget.AddToViewport` (`self.Inventory`) 0)))))

(event `Drink Stamina Potion`
  ;[1 1 1 1 100] Old Potion Invnetory System
  ;;[1 1 1] Doesnt get called on the animation. Maybe try addinga  New Emum (E_ConsumableType) with a switcher that checks what the potion is before calling on the heal player
  (`/Engine/EditorBlueprintResources/StandardMacros.DecrementInt` (`self.PotionQuantity`)
    (:`  `
      (`/Game/CombatFrameWork/Blueprints/Components/BP_Stats.RestorePlayerStamina` (`Actor.GetComponentByClass` (`self.GetOwner`) "/Game/CombatFrameWork/Blueprints/Components/BP_Stats.BP_Stats_C") (`self.PotionRestoreAmount`)))))

(event `Drink Potion`
  (bind _potionquantity (`self.PotionQuantity`))
  (bind _potionmesh (`self.PotionMesh`))
  ;[1 1 1 1 100] Old Potion Invnetory System
  (if (> _potionquantity 0)
    (bind _result (`/Engine/EditorBlueprintResources/StandardMacros.DecrementInt` _potionquantity)
      (:`  `
        (`KismetSystemLibrary.PrintString` (`KismetStringLibrary.Conv_IntToString` _result))
        (`/Game/CombatFrameWork/Blueprints/Components/BP_Stats.RestorePlayerHealth` (`Actor.GetComponentByClass` (`self.GetOwner`) "/Game/CombatFrameWork/Blueprints/Components/BP_Stats.BP_Stats_C") (`self.PotionRestoreAmount`))
        (`self.UpdateConsumables`)
        (`/Engine/EditorBlueprintResources/StandardMacros.IsValid` _potionmesh
          (:`Is Valid`
            (`/Game/CombatFrameWork/Blueprints/BP_Potion.Empty Glass` _potionmesh)))))))

(event `Drink Mana Potion`
  ;[1 1 1 1 100] Old Potion Invnetory System
  ;;[1 1 1] Doesnt get called on the animation. Maybe try addinga  New Emum (E_ConsumableType) with a switcher that checks what the potion is before calling on the heal player
  (`/Engine/EditorBlueprintResources/StandardMacros.DecrementInt` (`self.PotionQuantity`)
    (:`  `
      (`/Game/CombatFrameWork/Blueprints/Components/BP_Stats.RestorePlayerMana` (`Actor.GetComponentByClass` (`self.GetOwner`) "/Game/CombatFrameWork/Blueprints/Components/BP_Stats.BP_Stats_C") (`self.PotionRestoreAmount`)))))

(event `EnhancedInput|/Game/Inventory/Input/IA_CharacterSheet`
  (params (ActionValue :type Boolean) (ElapsedSeconds :type "Float (double-precision)") (TriggeredSeconds :type "Float (double-precision)") (InputAction :type "InputAction Object Reference" :default "/Game/Inventory/Input/IA_CharacterSheet.IA_CharacterSheet"))
  (bind _returnvalue (`GameplayStatics.GetPlayerController` 0))
  (bind _returnvalue_2 (`GameplayStatics.GetPlayerController` 0))
  ;[1 0 0] Loads equipment sheet Widget // bug with this not loading in the begining of the game //
  (:`Started`
    (if (`Widget.IsVisible` (`self.EquipmentSheet`))
      (if (not (`Widget.IsVisible` (`self.Inventory`)))
        (set `PlayerController.bShowMouseCursor` false _returnvalue)
        (`WidgetBlueprintLibrary.SetInputMode_GameOnly` _returnvalue))
      (`Widget.RemoveFromParent` (`self.EquipmentSheet`))
      (else
        (set `PlayerController.bShowMouseCursor` true _returnvalue_2)
        (`WidgetBlueprintLibrary.SetInputMode_GameAndUIEx` _returnvalue_2 (`self.EquipmentSheet`))
        (`UserWidget.AddToViewport` (`self.EquipmentSheet`) 0)))))

(event `Spawn Potion`
  (bind _returnvalue (`self.GetOwner`))
  ;[1 1 1 1 100] Old Potion Invnetory System
  (`/Game/CombatFrameWork/Blueprints/BP_Potion.Change Potion Mesh` (`self.PotionMesh`) (`self.Player Inventory`))
  (bind _returnvalue_2 (`|SpawnActorFromClass` "/Game/CombatFrameWork/Blueprints/BP_Potion.BP_Potion_C" (`Actor.GetTransform` _returnvalue) "AlwaysSpawn" "MultiplyWithRoot" null null))
  (bind _output_get (set `self.PotionMesh` _returnvalue_2))
  (`Actor.K2_AttachToComponent` _output_get (`Character.Mesh` (cast `Character` _returnvalue :!pure true)) (`self.Socket Name`) "SnapToTarget" "SnapToTarget" "KeepRelative" true))

(event `Despawn Potion`
  (bind _potionmesh (`self.PotionMesh`))
  ;[1 1 1 1 100] Old Potion Invnetory System
  (`/Engine/EditorBlueprintResources/StandardMacros.IsValid` _potionmesh
    (:`Is Valid`
      (`Actor.K2_DestroyActor` _potionmesh))))

(event `EnhancedInput|/Game/Inventory/Input/IA_save`
  (params (ActionValue :type Boolean) (ElapsedSeconds :type "Float (double-precision)") (TriggeredSeconds :type "Float (double-precision)") (InputAction :type "InputAction Object Reference" :default "/Game/Inventory/Input/IA_save.IA_save"))
  (bind _save_game (`self.Save Game`))
  (bind _equipmentsheet (`/Game/Inventory/Blueprints/BP_Inventory.EquipmentSheet` (`self.Player Inventory`)))
  (bind _equippeditems (`/Game/Inventory/Blueprints/BP_Save.EquippedItems` (`self.Save Game`)))
  ;[1 0 0] Save Game  keyboard 8
  (:`Started`
    (bind _returnvalue (`GameplayStatics.DoesSaveGameExist` "inventory"))
    (if _returnvalue
      (set `/Game/Inventory/Blueprints/BP_Save.Gear` (`self.GearSlots`) _save_game)
      (set `/Game/Inventory/Blueprints/BP_Save.Consumables` (`self.Consumable_Slots`) _save_game)
      (else
        (bind _returnvalue_2 (`GameplayStatics.CreateSaveGameObject` "/Game/Inventory/Blueprints/BP_Save.BP_Save_C"))
        (set `/Game/Inventory/Blueprints/BP_Save.Gear` (`self.GearSlots`) _returnvalue_2)
        (set `/Game/Inventory/Blueprints/BP_Save.Consumables` (`self.Consumable_Slots`) _returnvalue_2)))
    ;[1 0 0] Saves Equipment slots in character sheet
    (`KismetArrayLibrary.Array_Set` _equippeditems 0 (`/Game/Inventory/WidgetBlueprints/WB_EquipmentSlot.Item` (`/Game/Inventory/WidgetBlueprints/WB_EquipmentSheet.WB_HelmetEquipmentSlot` _equipmentsheet)) true)
    (`KismetArrayLibrary.Array_Set` _equippeditems 1 (`/Game/Inventory/WidgetBlueprints/WB_EquipmentSlot.Item` (`/Game/Inventory/WidgetBlueprints/WB_EquipmentSheet.WB_ChestEquipmentSlot` _equipmentsheet)) true)
    (`KismetArrayLibrary.Array_Set` _equippeditems 2 (`/Game/Inventory/WidgetBlueprints/WB_EquipmentSlot.Item` (`/Game/Inventory/WidgetBlueprints/WB_EquipmentSheet.WB_PantsEquipmentSlot` _equipmentsheet)) true)
    (`KismetArrayLibrary.Array_Set` _equippeditems 3 (`/Game/Inventory/WidgetBlueprints/WB_EquipmentSlot.Item` (`/Game/Inventory/WidgetBlueprints/WB_EquipmentSheet.WB_BootsEquipmentSlot` _equipmentsheet)) true)
    (`KismetArrayLibrary.Array_Set` _equippeditems 4 (`/Game/Inventory/WidgetBlueprints/WB_EquipmentSlot.Item` (`/Game/Inventory/WidgetBlueprints/WB_EquipmentSheet.WB_MainHandEquipmentSlot` _equipmentsheet)) true)
    (`KismetArrayLibrary.Array_Set` _equippeditems 5 (`/Game/Inventory/WidgetBlueprints/WB_EquipmentSlot.Item` (`/Game/Inventory/WidgetBlueprints/WB_EquipmentSheet.WB_OffhandEquipmentSlot` _equipmentsheet)) true)
    (`KismetArrayLibrary.Array_Set` _equippeditems 6 (`/Game/Inventory/WidgetBlueprints/WB_EquipmentSlot.Item` (`/Game/Inventory/WidgetBlueprints/WB_EquipmentSheet.WB_NecklaceEquipmentSlot` _equipmentsheet)) true)
    (`KismetArrayLibrary.Array_Set` _equippeditems 7 (`/Game/Inventory/WidgetBlueprints/WB_EquipmentSlot.Item` (`/Game/Inventory/WidgetBlueprints/WB_EquipmentSheet.WB_RingEquipmentSlot` _equipmentsheet)) true)
    (`KismetArrayLibrary.Array_Set` _equippeditems 8 (`/Game/Inventory/WidgetBlueprints/WB_EquipmentSlot.Item` (`/Game/Inventory/WidgetBlueprints/WB_EquipmentSheet.WB_EarringsEquipmentSlot` _equipmentsheet)) true)
    (`KismetArrayLibrary.Array_Set` _equippeditems 9 (`/Game/Inventory/WidgetBlueprints/WB_EquipmentSlot.Item` (`/Game/Inventory/WidgetBlueprints/WB_EquipmentSheet.WB_BeltEquipmentSlot` _equipmentsheet)) true)
    (`KismetArrayLibrary.Array_Set` _equippeditems 10 (`/Game/Inventory/WidgetBlueprints/WB_EquipmentSlot.Item` (`/Game/Inventory/WidgetBlueprints/WB_EquipmentSheet.WB_GlovesEquipmentSlot` _equipmentsheet)) true)
    (`KismetArrayLibrary.Array_Set` _equippeditems 11 (`/Game/Inventory/WidgetBlueprints/WB_EquipmentSlot.Item` (`/Game/Inventory/WidgetBlueprints/WB_EquipmentSheet.WB_BackEquipmentSlot` _equipmentsheet)) true)
    (`KismetArrayLibrary.Array_Set` _equippeditems 12 (`/Game/Inventory/WidgetBlueprints/WB_EquipmentSlot.Item` (`/Game/Inventory/WidgetBlueprints/WB_EquipmentSheet.WB_Pet` _equipmentsheet)) true)
    (`KismetArrayLibrary.Array_Set` _equippeditems 13 (`/Game/Inventory/WidgetBlueprints/WB_EquipmentSlot.Item` (`/Game/Inventory/WidgetBlueprints/WB_EquipmentSheet.WB_ConsumableSlot1` _equipmentsheet)) true)
    (`KismetArrayLibrary.Array_Set` _equippeditems 14 (`/Game/Inventory/WidgetBlueprints/WB_EquipmentSlot.Item` (`/Game/Inventory/WidgetBlueprints/WB_EquipmentSheet.WB_ConsumableSlot2` _equipmentsheet)) true)
    (`GameplayStatics.SaveGameToSlot` (`self.Save Game`) "inventory")
    (`KismetSystemLibrary.PrintString` "Saved")))

(event `Bonfire`
  ;[1 1 1 1 100] Old Potion Invnetory System
  (`self.UpdateConsumables`))

(event `EnhancedInput|/Game/Inventory/Input/IA_DELETESAVE`
  (params (ActionValue :type Boolean) (ElapsedSeconds :type "Float (double-precision)") (TriggeredSeconds :type "Float (double-precision)") (InputAction :type "InputAction Object Reference" :default "/Game/Inventory/Input/IA_DELETESAVE.IA_DELETESAVE"))
  ;[0.01938 0.01938 0.01938] Delete save keyboard 9
  (:`Started`
    (bind _returnvalue (`GameplayStatics.DeleteGameInSlot` "Inventory"))
    (if _returnvalue
      (`KismetArrayLibrary.Array_Clear` (`self.GearSlots`))
      (`KismetArrayLibrary.Array_Clear` (`self.Consumable_Slots`))
      (`KismetArrayLibrary.Array_Resize` (`self.GearSlots`) (`self.GearSlotSize`))
      (`KismetArrayLibrary.Array_Resize` (`self.Consumable_Slots`) (`self.ConsumableSlotSize`))
      (`/Game/Inventory/WidgetBlueprints/WB_ItemSlotInventory.LoadInventory` (`/Game/Inventory/WidgetBlueprints/WB_Inventory.WB_ItemInventory` (`self.Inventory`)) self)
      (`KismetSystemLibrary.PrintString` "save deleted"))))

(fn `AddItemToInventory`
  (params (Item :type "/Game/Inventory/Structures/S_ItemMaster Structure"))
  (returns (AddedItemToInventory :type Boolean))
  (bind (_datatable _itemtype) (break `/Game/Inventory/Structures/S_ItemMaster` (`local.Item`)))
  (bind (_datatable_2 _itemtype_2) (break `/Game/Inventory/Structures/S_ItemMaster` (`local.Item`)))
  (bind _wb_consumableslot1 (`/Game/Inventory/WidgetBlueprints/WB_EquipmentSheet.WB_ConsumableSlot1` (`self.EquipmentSheet`)))
  (bind _item (`/Game/Inventory/WidgetBlueprints/WB_EquipmentSlot.Item` (`/Game/Inventory/WidgetBlueprints/WB_EquipmentSheet.WB_ConsumableSlot1` (`self.EquipmentSheet`))))
  (bind (_datatable_3 _itemtype_3 _quantity) (break `/Game/Inventory/Structures/S_ItemMaster` _item))
  (bind _returnvalue (+ _quantity (`.Quantity_9_EBAE327348F95ABE9C9149A16AC0EA60` (break `/Game/Inventory/Structures/S_ItemMaster` (`local.Item`)))))
  (switch `/Game/Inventory/Enum/E_ItemType` (`.ItemType_5_FAB6B0534D36D6AB0807ACA423B8D793` (break `/Game/Inventory/Structures/S_ItemMaster` Item))
    (:`NewEnumerator0`
      ;[0.01938 0.01938 0.01938] Gear added
      (for (_array_element _array_index) (`self.GearSlots`)
        (if (== (`.Quantity_9_EBAE327348F95ABE9C9149A16AC0EA60` (break `/Game/Inventory/Structures/S_ItemMaster` _array_element)) 0)
          (`KismetArrayLibrary.Array_Set` (`self.GearSlots`) _array_index (`local.Item`))
          (return true)))
      (return false))
    (:`NewEnumerator2`
      ;[1 0.2057 0] This is used to auto Equip potions to the character sheet and add them to the total if it within the stacksize. Current Issue is will ad numbers lower than stacksize but if trying to add greater it creates a new stack. 4+4 = 2 stacks. 4+1=5, 4+2=6, 4+4= 4-4
      (if (> (`.Quantity_9_EBAE327348F95ABE9C9149A16AC0EA60` (break `/Game/Inventory/Structures/S_ItemMaster` (`/Game/Inventory/WidgetBlueprints/WB_EquipmentSlot.Item` (`/Game/Inventory/WidgetBlueprints/WB_EquipmentSheet.WB_ConsumableSlot1` (`self.EquipmentSheet`))))) 0)
        (if (== (`.RowName` (break `DataTableRowHandle` _datatable_3)) (`.RowName` (break `DataTableRowHandle` (`.DataTable_6_775A83664656B010A5EE4FBC86628E06` (break `/Game/Inventory/Structures/S_ItemMaster` (`local.Item`))))))
          (bind _returnvalue_2 (`|GetDataTableRow` "/Game/Inventory/DataTable/DataTable_Item.DataTable_Item" (`.RowName` (break `DataTableRowHandle` (`.DataTable_6_775A83664656B010A5EE4FBC86628E06` (break `/Game/Inventory/Structures/S_ItemMaster` _item)))))
            (:`then`
              (if (>= (`.StackSize_9_1E3505964A30451ACAB7199B2E765371` (break `/Game/Inventory/Structures/S_Item` _returnvalue_2)) _returnvalue)
                (bind _output_get (set `/Game/Inventory/WidgetBlueprints/WB_EquipmentSlot.Item` (make `/Game/Inventory/Structures/S_ItemMaster` _datatable_2 _itemtype_2 _returnvalue) _wb_consumableslot1))
                (`/Game/Inventory/WidgetBlueprints/WB_EquipmentSlot.UpdateSlot` _wb_consumableslot1 _output_get)
                (return true)
                (else
                  _))))))
      ;[1 1 1] Items not stacking right
      (for (_array_element_2 _array_index_2) (`self.Consumable_Slots`)
        (bind (_datatable_4 _itemtype_4 _quantity_2) (break `/Game/Inventory/Structures/S_ItemMaster` _array_element_2))
        (if (== (`.RowName` (break `DataTableRowHandle` _datatable_4)) (`.RowName` (break `DataTableRowHandle` (`.DataTable_6_775A83664656B010A5EE4FBC86628E06` (break `/Game/Inventory/Structures/S_ItemMaster` (`local.Item`))))))
          (bind _returnvalue_3 (`|GetDataTableRow` "/Game/Inventory/DataTable/DataTable_Item.DataTable_Item" (`.RowName` (break `DataTableRowHandle` (`.DataTable_6_775A83664656B010A5EE4FBC86628E06` (break `/Game/Inventory/Structures/S_ItemMaster` (`local.Item`))))))
            (:`then`
              (bind _returnvalue_4 (+ (`.Quantity_9_EBAE327348F95ABE9C9149A16AC0EA60` (break `/Game/Inventory/Structures/S_ItemMaster` (`local.Item`))) _quantity_2))
              (if (>= (`.StackSize_9_1E3505964A30451ACAB7199B2E765371` (break `/Game/Inventory/Structures/S_Item` _returnvalue_3)) _returnvalue_4)
                (`KismetArrayLibrary.Array_Set` (`self.Consumable_Slots`) _array_index_2 (make `/Game/Inventory/Structures/S_ItemMaster` _datatable _itemtype _returnvalue_4))
                (return true))))))
      (for (_array_element_3 _array_index_3) (`self.Consumable_Slots`)
        (if (== (`.Quantity_9_EBAE327348F95ABE9C9149A16AC0EA60` (break `/Game/Inventory/Structures/S_ItemMaster` _array_element_3)) 0)
          (`KismetArrayLibrary.Array_Set` (`self.Consumable_Slots`) _array_index_3 (`local.Item`))
          (return true)))
      (return false))))

(fn `CheckAmmo`)

(fn `Consume Consumable`
  (bind _potionmesh (`self.PotionMesh`))
  (bind _item (`/Game/Inventory/WidgetBlueprints/WB_EquipmentSlot.Item` (`/Game/Inventory/WidgetBlueprints/WB_EquipmentSheet.WB_ConsumableSlot1` (`self.EquipmentSheet`))))
  (bind (_datatable _itemtype _quantity) (break `/Game/Inventory/Structures/S_ItemMaster` _item))
  (if (> _quantity 0)
    (`/Engine/EditorBlueprintResources/StandardMacros.DecrementInt` _quantity
      (:`  `
        (bind _returnvalue (`|GetDataTableRow` "/Game/Inventory/DataTable/DataTable_Item.DataTable_Item" (`.RowName` (break `DataTableRowHandle` _datatable)))
          (:`then`
            ;[1 0 0] Change with a function that checks what the potion is the first (health, stamina, mana, other)
            (`/Game/CombatFrameWork/Blueprints/Components/BP_Stats.RestorePlayerHealth` (`Actor.GetComponentByClass` (`self.GetOwner`) "/Game/CombatFrameWork/Blueprints/Components/BP_Stats.BP_Stats_C") (`.RestoreAmount_38_429A496C413DAEEFA7F03D8360464038` (break `/Game/Inventory/Structures/S_Item` _returnvalue)))
            (`/Game/Inventory/WidgetBlueprints/WB_EquipmentSlot.UpdateSlot` (`/Game/Inventory/WidgetBlueprints/WB_EquipmentSheet.WB_ConsumableSlot1` (`self.EquipmentSheet`)) _item)
            (`self.UpdateConsumables`)
            (`/Engine/EditorBlueprintResources/StandardMacros.IsValid` _potionmesh
              (:`Is Valid`
                (`/Game/CombatFrameWork/Blueprints/BP_Potion.Empty Glass` _potionmesh)))))))))

(fn `Interact`
  (bind _returnvalue (- (`Actor.K2_GetActorLocation` (`GameplayStatics.GetPlayerCharacter` 0)) (0.0 0.0 30.0)))
  (bind _outhit (`KismetSystemLibrary.SphereTraceSingle` _returnvalue _returnvalue 120.0 "TraceTypeQuery1"))
  (bind (_bblockinghit _binitialoverlap _time _distance _location _impactpoint _normal _impactnormal _physmat _hitactor) (`GameplayStatics.BreakHitResult` _outhit))
  (if (`KismetSystemLibrary.DoesImplementInterface` _hitactor "/Game/CombatFrameWork/Blueprints/Interfaces/BP_Interact.BP_Interact_C")
    (message `/Game/CombatFrameWork/Blueprints/Interfaces/BP_Interact.Interact` _hitactor null self)))

(fn `LoadEquippedItems`
  (bind _equipmentsheet (`self.EquipmentSheet`))
  (`/Game/Inventory/WidgetBlueprints/WB_EquipmentSlot.UpdateSlot` (`/Game/Inventory/WidgetBlueprints/WB_EquipmentSheet.WB_HelmetEquipmentSlot` _equipmentsheet) (`|GetArrayItem` (`/Game/Inventory/Blueprints/BP_Save.EquippedItems` (`self.Save Game`))))
  (`/Game/Inventory/WidgetBlueprints/WB_EquipmentSlot.UpdateSlot` (`/Game/Inventory/WidgetBlueprints/WB_EquipmentSheet.WB_ChestEquipmentSlot` _equipmentsheet) (`|GetArrayItem` (`/Game/Inventory/Blueprints/BP_Save.EquippedItems` (`self.Save Game`)) 1))
  (`/Game/Inventory/WidgetBlueprints/WB_EquipmentSlot.UpdateSlot` (`/Game/Inventory/WidgetBlueprints/WB_EquipmentSheet.WB_PantsEquipmentSlot` _equipmentsheet) (`|GetArrayItem` (`/Game/Inventory/Blueprints/BP_Save.EquippedItems` (`self.Save Game`)) 2))
  (`/Game/Inventory/WidgetBlueprints/WB_EquipmentSlot.UpdateSlot` (`/Game/Inventory/WidgetBlueprints/WB_EquipmentSheet.WB_BootsEquipmentSlot` _equipmentsheet) (`|GetArrayItem` (`/Game/Inventory/Blueprints/BP_Save.EquippedItems` (`self.Save Game`)) 3))
  (`/Game/Inventory/WidgetBlueprints/WB_EquipmentSlot.UpdateSlot` (`/Game/Inventory/WidgetBlueprints/WB_EquipmentSheet.WB_MainHandEquipmentSlot` _equipmentsheet) (`|GetArrayItem` (`/Game/Inventory/Blueprints/BP_Save.EquippedItems` (`self.Save Game`)) 4))
  (`/Game/Inventory/WidgetBlueprints/WB_EquipmentSlot.UpdateSlot` (`/Game/Inventory/WidgetBlueprints/WB_EquipmentSheet.WB_OffhandEquipmentSlot` _equipmentsheet) (`|GetArrayItem` (`/Game/Inventory/Blueprints/BP_Save.EquippedItems` (`self.Save Game`)) 5))
  (`/Game/Inventory/WidgetBlueprints/WB_EquipmentSlot.UpdateSlot` (`/Game/Inventory/WidgetBlueprints/WB_EquipmentSheet.WB_NecklaceEquipmentSlot` _equipmentsheet) (`|GetArrayItem` (`/Game/Inventory/Blueprints/BP_Save.EquippedItems` (`self.Save Game`)) 6))
  (`/Game/Inventory/WidgetBlueprints/WB_EquipmentSlot.UpdateSlot` (`/Game/Inventory/WidgetBlueprints/WB_EquipmentSheet.WB_RingEquipmentSlot` _equipmentsheet) (`|GetArrayItem` (`/Game/Inventory/Blueprints/BP_Save.EquippedItems` (`self.Save Game`)) 7))
  (`/Game/Inventory/WidgetBlueprints/WB_EquipmentSlot.UpdateSlot` (`/Game/Inventory/WidgetBlueprints/WB_EquipmentSheet.WB_EarringsEquipmentSlot` _equipmentsheet) (`|GetArrayItem` (`/Game/Inventory/Blueprints/BP_Save.EquippedItems` (`self.Save Game`)) 8))
  (`/Game/Inventory/WidgetBlueprints/WB_EquipmentSlot.UpdateSlot` (`/Game/Inventory/WidgetBlueprints/WB_EquipmentSheet.WB_BeltEquipmentSlot` _equipmentsheet) (`|GetArrayItem` (`/Game/Inventory/Blueprints/BP_Save.EquippedItems` (`self.Save Game`)) 9))
  (`/Game/Inventory/WidgetBlueprints/WB_EquipmentSlot.UpdateSlot` (`/Game/Inventory/WidgetBlueprints/WB_EquipmentSheet.WB_GlovesEquipmentSlot` _equipmentsheet) (`|GetArrayItem` (`/Game/Inventory/Blueprints/BP_Save.EquippedItems` (`self.Save Game`)) 10))
  (`/Game/Inventory/WidgetBlueprints/WB_EquipmentSlot.UpdateSlot` (`/Game/Inventory/WidgetBlueprints/WB_EquipmentSheet.WB_BackEquipmentSlot` _equipmentsheet) (`|GetArrayItem` (`/Game/Inventory/Blueprints/BP_Save.EquippedItems` (`self.Save Game`)) 11))
  (`/Game/Inventory/WidgetBlueprints/WB_EquipmentSlot.UpdateSlot` (`/Game/Inventory/WidgetBlueprints/WB_EquipmentSheet.WB_Pet` _equipmentsheet) (`|GetArrayItem` (`/Game/Inventory/Blueprints/BP_Save.EquippedItems` (`self.Save Game`)) 12))
  (`/Game/Inventory/WidgetBlueprints/WB_EquipmentSlot.UpdateSlot` (`/Game/Inventory/WidgetBlueprints/WB_EquipmentSheet.WB_ConsumableSlot1` _equipmentsheet) (`|GetArrayItem` (`/Game/Inventory/Blueprints/BP_Save.EquippedItems` (`self.Save Game`)) 13))
  (`/Game/Inventory/WidgetBlueprints/WB_EquipmentSlot.UpdateSlot` (`/Game/Inventory/WidgetBlueprints/WB_EquipmentSheet.WB_ConsumableSlot2` _equipmentsheet) (`|GetArrayItem` (`/Game/Inventory/Blueprints/BP_Save.EquippedItems` (`self.Save Game`)) 14)))