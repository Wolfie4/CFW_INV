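; Anim notify state that switches rotation on for a window of an animation in the combat framework.
; On begin it finds the BP_Rotating component on the mesh owner and, if valid, calls ToggleRotation with true.
; On end it calls ToggleRotation with false on the same component, so the animation timeline controls when the owner may rotate.
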(fn `Received_NotifyBegin`
  (params (MeshComp :type "SkeletalMeshComponent Object Reference") (Animation :type "AnimSequenceBase Object Reference") (TotalDuration :type "Float (single-precision)") (EventReference :type "AnimNotifyEventReference Structure (by ref)"))
  (returns (ReturnValue :type Boolean))
  (bind _returnvalue (`Actor.GetComponentByClass` (`ActorComponent.GetOwner` MeshComp) "/Game/CombatFrameWork/Blueprints/Components/BP_Rotating.BP_Rotating_C"))
  (`/Engine/EditorBlueprintResources/StandardMacros.IsValid` _returnvalue
    (:`Is Valid`
      (`/Game/CombatFrameWork/Blueprints/Components/BP_Rotating.Toggle Rotation` _returnvalue true)
      (return true))))

(fn `Received_NotifyEnd`
  (params (MeshComp :type "SkeletalMeshComponent Object Reference") (Animation :type "AnimSequenceBase Object Reference") (EventReference :type "AnimNotifyEventReference Structure (by ref)"))
  (returns (ReturnValue :type Boolean))
  (bind _returnvalue (`Actor.GetComponentByClass` (`ActorComponent.GetOwner` MeshComp) "/Game/CombatFrameWork/Blueprints/Components/BP_Rotating.BP_Rotating_C"))
  (`/Engine/EditorBlueprintResources/StandardMacros.IsValid` _returnvalue
    (:`Is Valid`
      (`/Game/CombatFrameWork/Blueprints/Components/BP_Rotating.Toggle Rotation` _returnvalue false)
      (return true))))