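; Base armor equipment actor that provides a worn skeletal mesh and a defense bonus to the owning character.
; Equipping attaches the mesh to the character's mesh as leader pose so it follows the body animation, then raises defense in BP_Stats by DefenseAmount.
; Unequipping lowers defense and detaches the mesh, though it also re-runs the attach step first.
; The attach function ignores its socket name input.
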(fn `Attach To Player`
  (params (SocketName :type Name))
  (bind _skeletalmesh (`self.SkeletalMesh`))
  (bind _mesh (`Character.Mesh` (cast `Character` (`self.GetOwner`) :!pure true)))
  (`/Engine/EditorBlueprintResources/StandardMacros.IsValid` (`SkeletalMeshComponent.SkeletalMeshAsset` (`self.SkeletalMesh`))
    (:`Is Valid`
      (`SceneComponent.K2_AttachToComponent` _skeletalmesh _mesh "None" "SnapToTarget" "SnapToTarget" "SnapToTarget" true)
      (`SkinnedMeshComponent.SetLeaderPoseComponent` _skeletalmesh _mesh false false))))

(fn `Equip Item`
  (`self.Attach To Player` "None")
  (`/Game/CombatFrameWork/Blueprints/Components/BP_Stats.IncreaseDefense` (`self.GetComponentByClass` (`self.GetOwner`) "/Game/CombatFrameWork/Blueprints/Components/BP_Stats.BP_Stats_C") (`self.DefenseAmount`)))

(fn `Unequip Item`
  (`self.Attach To Player` "None")
  (`/Game/CombatFrameWork/Blueprints/Components/BP_Stats.DecreaseDefense` (`self.GetComponentByClass` (`self.GetOwner`) "/Game/CombatFrameWork/Blueprints/Components/BP_Stats.BP_Stats_C") (`self.DefenseAmount`))
  (`SceneComponent.K2_DetachFromComponent` (`self.SkeletalMesh`) "KeepWorld" "KeepWorld" "KeepWorld" true))

(fn `UserConstructionScript`
  (`parent.UserConstructionScript`))