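; Boss enemy that extends a parent AI character with a great hammer, screen-space health bar and theme music.
; Stats feed the boss HUD, shown on sighting a target as music starts once.
; Collision toggle events arm the hammer trace, which damages only the player.
; Death drops the hammer as physics, shows a defeated screen and, if music exists, fades it and destroys the boss after a delay.
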(event `self.ReceiveBeginPlay`
  (`parent.ReceiveBeginPlay`)
  (`/Game/CombatFrameWork/Blueprints/Components/BP_Collision.Set Weapon` (`self.BP_Collision1`) (`self.GreatHamemr`))
  (`ActorComponent.K2_DestroyComponent` (`self.Healthbar`))
  (bind _returnvalue (`|CreateWidget` "/Game/CombatFrameWork/Blueprints/Widgets/WB_BossHealthBar.WB_BossHealthBar_C"))
  (bind _output_get (set `self.BossHUD` _returnvalue))
  (`UserWidget.AddToViewport` _output_get 0)
  (`/Game/CombatFrameWork/Blueprints/Widgets/WB_BossHealthBar.Set stat bar ref` (`self.BossHUD`) (`self.BP_Stats`)))

(event `self.ReceiveTick`
  (params (DeltaSeconds :type "Float (single-precision)"))
  (`parent.ReceiveTick` DeltaSeconds))

(event `self.BP_Collision1.Damage Actor`
  (params (`Hit Data` :type "HitResult Structure"))
  (bind (_bblockinghit _binitialoverlap _time _distance _location _impactpoint _normal _impactnormal _physmat _hitactor) (`GameplayStatics.BreakHitResult` `Hit Data`))
  (bind _returnvalue (`self.GetOwner`))
  ;[1 1 1] Enemy can only damage the player
  (if (== _hitactor (`GameplayStatics.GetPlayerCharacter` 0))
    (`GameplayStatics.ApplyPointDamage` _hitactor (`self.Calculate Damage`) (`self.GetActorForwardVector` _returnvalue) `Hit Data` (`self.GetInstigatorController` _returnvalue) null "/Game/CombatFrameWork/Blueprints/Damage/BP_DamageType.BP_DamageType_C")))

(event `/Game/CombatFrameWork/Blueprints/Interfaces/BP_Combat.ActivateCollision`
  (params (CollisionType :type "/Game/CombatFrameWork/Blueprints/Enums/E_CollisionType Enum" :default "NewEnumerator0"))
  (switch `/Game/CombatFrameWork/Blueprints/Enums/E_CollisionType` CollisionType
    (:`NewEnumerator0`
      (`/Game/CombatFrameWork/Blueprints/Components/BP_Collision.Turn On Collision` (`self.BP_Collision1`)))))

(event `/Game/CombatFrameWork/Blueprints/Interfaces/BP_Combat.DeactivateCollision`
  (`/Game/CombatFrameWork/Blueprints/Components/BP_Collision.Turn Off Colliison` (`self.BP_Collision1`)))

(event `self.Sees Target`
  (params (Actor :type "Actor Object Reference"))
  ;[0.01938 0.01938 0.01938] See player starts fight music and hud
  (`/Engine/EditorBlueprintResources/StandardMacros.IsValid` Actor
    (:`Is Valid`
      (`Widget.SetVisibility` (`self.BossHUD`) "Visible")
      (`/Engine/EditorBlueprintResources/StandardMacros.DoOnce` false
        (:`Completed`
          (bind _returnvalue (`GameplayStatics.SpawnSound2D` "/Game/CombatFrameWork/SFX/BossMusic/SW_Bosstheme.SW_Bosstheme" 0.2 1.0 0.0 null))
          (bind _output_get (set `self.Bossmusic` _returnvalue))
          (`AudioComponent.FadeIn` _output_get 1.0 1.0 0.0 "Linear"))))))

(event `self.BP_Stats.Death`
  (bind _bossmusic (`self.Bossmusic`))
  (bind _greathamemr (`self.GreatHamemr`))
  ;[0.01938 0.01938 0.01938] Death
  (`/Engine/EditorBlueprintResources/StandardMacros.DoOnce` false
    (:`Completed`
      (`self.StopAnimMontage` null)
      (`Widget.RemoveFromParent` (`self.BossHUD`))
      (`SceneComponent.K2_DetachFromComponent` _greathamemr "KeepWorld" "KeepWorld" "KeepWorld" true)
      (`PrimitiveComponent.SetCollisionEnabled` _greathamemr "QueryAndPhysics")
      (`PrimitiveComponent.SetSimulatePhysics` _greathamemr true)
      ;;[0.01938 0.01938 0.01938] Boss defeated Screen
      (`/Engine/EditorBlueprintResources/StandardMacros.DoOnce` false
        (:`Completed`
          (bind _returnvalue (`|CreateWidget` "/Game/CombatFrameWork/Blueprints/Widgets/WB_BossDefeated.WB_BossDefeated_C"))
          (`UserWidget.AddToViewport` _returnvalue 0)
          (`/Engine/EditorBlueprintResources/StandardMacros.IsValid` _bossmusic
            (:`Is Valid`
              (`AudioComponent.FadeOut` _bossmusic 10.0 0.0 "Linear")
              (`/Game/CombatFrameWork/Blueprints/Components/BP_Collision.Turn Off Colliison` (`self.BP_Collision`))
              (`/Game/CombatFrameWork/Blueprints/Components/BP_Collision.Turn Off Colliison` (`self.BP_Collision1`))
              ;;[1 0.8098 0] Add dissolve or emitter on death
              (`KismetSystemLibrary.Delay` 10.0)
              (`self.K2_DestroyActor`))))))))

(fn `UserConstructionScript`
  (`parent.UserConstructionScript`))