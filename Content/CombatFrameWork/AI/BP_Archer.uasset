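; BP_Archer is an enemy archer character that shoots arrows at the player, extending a parent combat character.
; On BeginPlay it spawns a bow attached to its hand socket, and ShootArrow plays the shoot-and-draw montage unless stunned.
; DrawBow and FireArrow animate the string and toggle the held arrow mesh, with FireArrow launching a spawned arrow toward the player.
; A switchable collision component applies point damage only to the player.
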(event `self.ReceiveBeginPlay`
  (`parent.ReceiveBeginPlay`)
  (bind _returnvalue (`|SpawnActorFromClass` "/Game/CombatFrameWork/Blueprints/Equipment/BP_BaseBow.BP_BaseBow_C" (`KismetMathLibrary.MakeTransform` (0.0 0.0 0.0)) "Undefined" "MultiplyWithRoot" null "/Game/CombatFrameWork/SFX/Impact/A_HitSound.A_HitSound" null))
  (bind _output_get (set `self.Bow Reference` _returnvalue))
  (`self.K2_AttachToComponent` _output_get (`self.Mesh`) "BowUse" "SnapToTarget" "SnapToTarget" "SnapToTarget" true))

(event `self.BP_Collision1.Damage Actor`
  (params (`Hit Data` :type "HitResult Structure"))
  (bind (_bblockinghit _binitialoverlap _time _distance _location _impactpoint _normal _impactnormal _physmat _hitactor) (`GameplayStatics.BreakHitResult` `Hit Data`))
  (bind _returnvalue (`self.GetOwner`))
  ;[1 1 1] Enemy can only damage the player
  (if (== _hitactor (`GameplayStatics.GetPlayerCharacter` 0))
    (`GameplayStatics.ApplyPointDamage` _hitactor (`self.Calculate Damage`) (`self.GetActorForwardVector` _returnvalue) `Hit Data` (`self.GetInstigatorController` _returnvalue) null "/Game/CombatFrameWork/Blueprints/Damage/BP_DamageType.BP_DamageType_C")))

(event `self.ActivateCollision`
  (params (CollisionType :type "/Game/CombatFrameWork/Blueprints/Enums/E_CollisionType Enum" :default "NewEnumerator0"))
  (switch `/Game/CombatFrameWork/Blueprints/Enums/E_CollisionType` CollisionType
    (:`NewEnumerator0`
      (`/Game/CombatFrameWork/Blueprints/Components/BP_Collision.Turn On Collision` (`self.BP_Collision1`)))))

(event `self.DeactivateCollision`
  (`/Game/CombatFrameWork/Blueprints/Components/BP_Collision.Turn Off Colliison` (`self.BP_Collision1`)))

(event `/Game/CombatFrameWork/Blueprints/Interfaces/BP_Combat.ShootArrow`
  (if (!= (`/Game/CombatFrameWork/Blueprints/Components/BP_State.Current State` (`self.BP_State`)) (struct :`TagName` "Player.State.Stunned"))
    (`self.PlayAnimMontage` "/Game/CombatFrameWork/Animations/Archer/AR_ShootAndDraw_Montage_Enemy.AR_ShootAndDraw_Montage_Enemy")))

(event `FIreArrow`
  (bind _arrowspawn (`self.ArrowSpawn`))
  (bind _returnvalue (`|SpawnActorFromClass` "/Game/CombatFrameWork/Blueprints/Equipment/BP_ArrowBase.BP_ArrowBase_C" (`KismetMathLibrary.MakeTransform` (`SceneComponent.K2_GetComponentLocation` _arrowspawn) (`SceneComponent.K2_GetComponentRotation` _arrowspawn)) "Undefined" "MultiplyWithRoot" self null))
  (`/Game/CombatFrameWork/Blueprints/Equipment/BP_ArrowBase.FireArrow` _returnvalue (`KismetMathLibrary.GetDirectionUnitVector` (`self.K2_GetActorLocation`) (`self.K2_GetActorLocation` (`GameplayStatics.GetPlayerCharacter` 0))))
  (`/Game/CombatFrameWork/Blueprints/Equipment/BP_BaseBow.Release String` (`self.Bow Reference`))
  (`SceneComponent.SetVisibility` (`self.SM_Arrow`) false false))

(event `/Game/CombatFrameWork/Blueprints/Interfaces/BP_Combat.DrawBow`
  (`/Game/CombatFrameWork/Blueprints/Equipment/BP_BaseBow.DrawString` (`self.Bow Reference`))
  (`SceneComponent.SetVisibility` (`self.SM_Arrow`) true false))

(fn `UserConstructionScript`
  (`parent.UserConstructionScript`))