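; Lock-on targeting component for a Character, with toggling and left/right target switching.
; A sphere trace gathers targetable interface actors, then line traces and camera-forward dot products pick the most centred one.
; Side switching splits candidates by hit normal against the camera's right vector.
; While locked, Tick interpolates control rotation toward a point below the target, releasing it when out of range or untargetable.
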(event `self.ReceiveBeginPlay`
  ;[0.01938 0.01938 0.01938] Getting References
  (bind _ascharacter (cast `Character` (`self.GetOwner`)))
  (set `self.Character Ref` _ascharacter)
  (set `self.Camera Ref` (`Actor.GetComponentByClass` (`self.Character Ref`) "/Script/Engine.CameraComponent")))

(event `Lock On Target`
  (bind _closesttarget (`self.Find Closest Target` (`self.Find Lock On Targets`)))
  ;[0.01938 0.01938 0.01938] Checks Closest Targets and locks camera to them
  (`/Engine/EditorBlueprintResources/StandardMacros.IsValid` _closesttarget
    (:`Is Valid`
      (bind _output_get (set `self.LockonTarget` _closesttarget))
      (message `/Game/CombatFrameWork/Blueprints/Interfaces/BP_Targeting.OnTargeted` _output_get true)
      (`self.Orient Camera`)
      (set `self.LockedOn?` true))))

(event `self.ReceiveTick`
  (params (DeltaSeconds :type "Float (single-precision)"))
  ;[0.01938 0.01938 0.01938] When Locked onto a Target Orients camera to then, Tilts Down and disables free look camera. Leaving Range of Target Disables Lock on
  (if (`self.LockedOn?`)
    (bind _returnvalue (message `/Game/CombatFrameWork/Blueprints/Interfaces/BP_Targeting.CanBeTargeted` (`self.LockonTarget`)))
    (if (or (not _returnvalue) (> (`KismetMathLibrary.Vector_Distance` (`Actor.K2_GetActorLocation` (`self.Character Ref`)) (`Actor.K2_GetActorLocation` (`self.LockonTarget`))) (`self.Tageting Radius`)))
      (`self.Stop Lock on`)
      (else
        (`self.Face Locked On Actor`)))))

(event `Toggle Lockon`
  ;[0.01938 0.01938 0.01938] Toggle on / off Check
  (if (`self.LockedOn?`)
    (`self.Stop Lock on`)
    (else
      (`self.Lock On Target`))))

(event `Stop Lock on`
  ;[0.01938 0.01938 0.01938] When Lock on Ends. Resets Player orientation
  (message `/Game/CombatFrameWork/Blueprints/Interfaces/BP_Targeting.OnTargeted` (`self.LockonTarget`) false)
  (set `self.LockonTarget` null)
  (set `self.LockedOn?` false)
  (`self.Orient Movement`))

(event `Switch To Left Locked on actor`
  (bind _closesttarget (`self.Find Closest Target On Left` (`self.Find Lock On Targets`)))
  ;[0.02315 0.02315 0.02315] Locks Left Target
  (`/Engine/EditorBlueprintResources/StandardMacros.IsValid` (`self.LockonTarget`)
    (:`Is Valid`
      (message `/Game/CombatFrameWork/Blueprints/Interfaces/BP_Targeting.OnTargeted` (`self.LockonTarget`) false)
      (`/Engine/EditorBlueprintResources/StandardMacros.IsValid` _closesttarget
        (:`Is Valid`
          (set `self.LockonTarget` _closesttarget)
          (message `/Game/CombatFrameWork/Blueprints/Interfaces/BP_Targeting.OnTargeted` (`self.LockonTarget`) true))))))

(event `Switch To RIght Locked On Actor`
  (bind _closesttarget (`self.Find Closest Target On Right` (`self.Find Lock On Targets`)))
  ;[0.02315 0.02315 0.02315] Locks Right Target
  (`/Engine/EditorBlueprintResources/StandardMacros.IsValid` (`self.LockonTarget`)
    (:`Is Valid`
      (message `/Game/CombatFrameWork/Blueprints/Interfaces/BP_Targeting.OnTargeted` (`self.LockonTarget`) false)
      (`/Engine/EditorBlueprintResources/StandardMacros.IsValid` _closesttarget
        (:`Is Valid`
          (set `self.LockonTarget` _closesttarget)
          (message `/Game/CombatFrameWork/Blueprints/Interfaces/BP_Targeting.OnTargeted` (`self.LockonTarget`) true))))))

(fn `Check How Close Target Is To Player`
  (params (Actor :type "Actor Object Reference"))
  (returns (ReturnValue :type "Float (double-precision)"))
  (return (`KismetMathLibrary.Dot_VectorVector` (`SceneComponent.GetForwardVector` (`self.Camera Ref`)) (`KismetMathLibrary.Conv_RotatorToVector` (`KismetMathLibrary.FindLookAtRotation` (`Actor.K2_GetActorLocation` (`self.Character Ref`)) (`Actor.K2_GetActorLocation` Actor))))))

(fn `Face Locked On Actor`
  (bind _returnvalue (`Actor.K2_GetActorRotation` (`Pawn.GetController` (`self.Character Ref`))))
  (bind (_returnvalue_roll _returnvalue_pitch _returnvalue_yaw) (`KismetMathLibrary.BreakRotator` (`KismetMathLibrary.RInterpTo` _returnvalue (`KismetMathLibrary.FindLookAtRotation` (`Actor.K2_GetActorLocation` (`self.GetOwner`)) (- (`Actor.K2_GetActorLocation` (`self.LockonTarget`)) (0.0 0.0 200.0))) (`GameplayStatics.GetWorldDeltaSeconds`) (`self.Target Rotation Speed`))))
  (`Controller.SetControlRotation` (`Pawn.GetController` (`self.Character Ref`)) (`KismetMathLibrary.MakeRotator` (.roll _returnvalue) _returnvalue_pitch _returnvalue_yaw)))

(fn `Find Closest Target`
  (params (Targets :type "Array of Actor Object Reference"))
  (returns (ClosestTarget :type "Actor Object Reference"))
  (locals (LocalTargetCompateValue :type "Float (double-precision)") (LocalClosestTarget :type "Actor Object Reference"))
  (for _array_element Targets
    (bind (_outhit _returnvalue) (`KismetSystemLibrary.LineTraceSingle` (`SceneComponent.K2_GetComponentLocation` (`self.Camera Ref`)) (`Actor.K2_GetActorLocation` _array_element) "TraceTypeQuery1"))
    (if _returnvalue
      (bind _returnvalue_2 (`self.Check How Close Target Is To Player` _array_element))
      (`/Engine/EditorBlueprintResources/StandardMacros.CompareFloat` _returnvalue_2 (`local.LocalTargetCompateValue`)
        (:`>`
          (set `local.LocalTargetCompateValue` _returnvalue_2)
          (set `local.LocalClosestTarget` _array_element)))))
  (return (`local.LocalClosestTarget`)))

(fn `Find Closest Target On Left`
  (params (Targets :type "Array of Actor Object Reference"))
  (returns (ClosestTarget :type "Actor Object Reference"))
  (locals (LocalTargetCompateValue :type "Float (double-precision)") (LocalClosestTarget :type "Actor Object Reference"))
  (for _array_element Targets
    (bind (_outhit _returnvalue) (`KismetSystemLibrary.LineTraceSingle` (`SceneComponent.K2_GetComponentLocation` (`self.Camera Ref`)) (`Actor.K2_GetActorLocation` _array_element) "TraceTypeQuery1"))
    (if (and (!= _array_element (`self.LockonTarget`)) _returnvalue (> (`KismetMathLibrary.Dot_VectorVector` (`SceneComponent.GetRightVector` (`self.Camera Ref`)) (`.Normal` (`GameplayStatics.BreakHitResult` _outhit))) 0.0))
      (if _returnvalue
        (bind _returnvalue_2 (`self.Check How Close Target Is To Player` _array_element))
        (`/Engine/EditorBlueprintResources/StandardMacros.CompareFloat` _returnvalue_2 (`local.LocalTargetCompateValue`)
          (:`>`
            (set `local.LocalTargetCompateValue` _returnvalue_2)
            (set `local.LocalClosestTarget` _array_element))))))
  (return (`local.LocalClosestTarget`)))

(fn `Find Closest Target On Right`
  (params (Targets :type "Array of Actor Object Reference"))
  (returns (ClosestTarget :type "Actor Object Reference"))
  (locals (LocalTargetCompateValue :type "Float (double-precision)") (LocalClosestTarget :type "Actor Object Reference"))
  (for _array_element Targets
    (bind (_outhit _returnvalue) (`KismetSystemLibrary.LineTraceSingle` (`SceneComponent.K2_GetComponentLocation` (`self.Camera Ref`)) (`Actor.K2_GetActorLocation` _array_element) "TraceTypeQuery1"))
    (if (and (!= _array_element (`self.LockonTarget`)) _returnvalue (< (`KismetMathLibrary.Dot_VectorVector` (`SceneComponent.GetRightVector` (`self.Camera Ref`)) (`.Normal` (`GameplayStatics.BreakHitResult` _outhit))) 0.0))
      (if _returnvalue
        (bind _returnvalue_2 (`self.Check How Close Target Is To Player` _array_element))
        (`/Engine/EditorBlueprintResources/StandardMacros.CompareFloat` _returnvalue_2 (`local.LocalTargetCompateValue`)
          (:`>`
            (set `local.LocalTargetCompateValue` _returnvalue_2)
            (set `local.LocalClosestTarget` _array_element))))))
  (return (`local.LocalClosestTarget`)))

(fn `Find Lock On Targets`
  (returns (`Potential Lockon Targets` :type "Array of Actor Object Reference"))
  (locals (TargetingActors :type "Array of Actor Object Reference"))
  (bind _returnvalue (`Actor.K2_GetActorLocation` (`self.Character Ref`)))
  (bind (_outhits _returnvalue_2) (`KismetSystemLibrary.SphereTraceMultiForObjects` _returnvalue _returnvalue (`self.Tageting Radius`) (`|MakeArray` "ObjectTypeQuery8" :!type "EObjectTypeQuery Enum") false (`|MakeArray` (`self.GetOwner`))))
  (for _array_element _outhits
    (if _returnvalue_2
      (bind (_bblockinghit _binitialoverlap _time _distance _location _impactpoint _normal _impactnormal _physmat _hitactor) (`GameplayStatics.BreakHitResult` _array_element))
      (bind _returnvalue_3 (message `/Game/CombatFrameWork/Blueprints/Interfaces/BP_Targeting.CanBeTargeted` _hitactor))
      (if (and _returnvalue_3 (`KismetSystemLibrary.DoesImplementInterface` _hitactor "/Game/CombatFrameWork/Blueprints/Interfaces/BP_Targeting.BP_Targeting_C"))
        (`KismetArrayLibrary.Array_Add` (`local.TargetingActors`) _hitactor))))
  (return (`local.TargetingActors`)))

(fn `Orient Camera`
  (bind _charactermovement (`Character.CharacterMovement` (`self.Character Ref`)))
  (set `CharacterMovementComponent.bOrientRotationToMovement` false _charactermovement)
  (set `CharacterMovementComponent.bUseControllerDesiredRotation` true _charactermovement))

(fn `Orient Movement`
  (bind _charactermovement (`Character.CharacterMovement` (`self.Character Ref`)))
  (set `CharacterMovementComponent.bOrientRotationToMovement` true _charactermovement)
  (set `CharacterMovementComponent.bUseControllerDesiredRotation` false _charactermovement))