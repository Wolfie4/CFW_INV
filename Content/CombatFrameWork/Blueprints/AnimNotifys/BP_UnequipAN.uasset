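; Anim notify that sheathes the owner's equipment at the notify's point in an animation.
; It tells the owner's BP_Combat component to toggle equipment off, disables combat and attaches the main weapon to its unequipped socket.
; If a valid main shield exists and the weapon's combat type matches one specific enum value, the shield also moves to its unequipped socket.
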(fn `Received_Notify`
  (params (MeshComp :type "SkeletalMeshComponent Object Reference") (Animation :type "AnimSequenceBase Object Reference") (EventReference :type "AnimNotifyEventReference Structure (by ref)"))
  (returns (ReturnValue :type Boolean))
  (bind _returnvalue (`Actor.GetComponentByClass` (`ActorComponent.GetOwner` MeshComp) "/Game/CombatFrameWork/Blueprints/Components/BP_Combat.BP_Combat_C"))
  (bind _mainweapon (`/Game/CombatFrameWork/Blueprints/Components/BP_Combat.MainWeapon` _returnvalue))
  (bind _mainshield (`/Game/CombatFrameWork/Blueprints/Components/BP_Combat.MainShield` _returnvalue))
  (`/Game/CombatFrameWork/Blueprints/Components/BP_Combat.ToggleEquipment` _returnvalue false)
  (set `/Game/CombatFrameWork/Blueprints/Components/BP_Combat.CombatEnabled?` false _returnvalue)
  (`/Game/CombatFrameWork/Blueprints/Equipment/BP_BaseEquipment.Attach To Player` _mainweapon (`/Game/CombatFrameWork/Blueprints/Equipment/BP_BaseWeapon.UnequippedSocket` _mainweapon))
  (`/Engine/EditorBlueprintResources/StandardMacros.IsValid` _mainshield
    (:`Is Valid`
      (if (`|EnumEquality` (`/Game/CombatFrameWork/Blueprints/Equipment/BP_BaseWeapon.CombatType` _mainweapon) "NewEnumerator1")
        (`/Game/CombatFrameWork/Blueprints/Equipment/BP_BaseEquipment.Attach To Player` _mainshield (`/Game/CombatFrameWork/Blueprints/Equipment/BP_BaseShield.UnequippedSocket` _mainshield))
        (return true)
        (else
          (return true))))
    (:`Is Not Valid`
      (return true))))