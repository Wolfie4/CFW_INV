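; BP_Chest is a lootable chest that highlights itself and shows an interact widget while the player character is inside its sphere.
; Interact adds a loot bar widget, created at BeginPlay with a reference to the chest, and plays a timeline that pitches the Cube component open.
; A close event reverses that timeline, and Removeitem blanks a slot in the chest's item array by index.
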(event `self.ReceiveBeginPlay`
  (bind _returnvalue (`|CreateWidget` "/Game/Inventory/WidgetBlueprints/WB_Lootbar.WB_Lootbar_C" null self))
  (set `self.LootbarWidget` _returnvalue))

(event `self.Sphere.OnComponentBeginOverlap`
  (params (OverlappedComponent :type "PrimitiveComponent Object Reference") (OtherActor :type "Actor Object Reference") (OtherComp :type "PrimitiveComponent Object Reference") (OtherBodyIndex :type Integer) (bFromSweep :type Boolean) (SweepResult :type "HitResult Structure (by ref)"))
  (if (== OtherActor (`GameplayStatics.GetPlayerCharacter` 0))
    (`MeshComponent.SetOverlayMaterial` (`self.Chest_Bottom`) "/Game/Inventory/Materials/M_Outline_InstTest.M_Outline_InstTest")
    (`MeshComponent.SetOverlayMaterial` (`self.Chest_Top`) "/Game/Inventory/Materials/M_Outline_InstTest.M_Outline_InstTest")
    (`SceneComponent.SetVisibility` (`self.W_Interact`) true false)))

(event `self.Sphere.OnComponentEndOverlap`
  (params (OverlappedComponent :type "PrimitiveComponent Object Reference") (OtherActor :type "Actor Object Reference") (OtherComp :type "PrimitiveComponent Object Reference") (OtherBodyIndex :type Integer))
  (if (== OtherActor (`GameplayStatics.GetPlayerCharacter` 0))
    (`MeshComponent.SetOverlayMaterial` (`self.Chest_Bottom`) null)
    (`MeshComponent.SetOverlayMaterial` (`self.Chest_Top`) null)
    (`SceneComponent.SetVisibility` (`self.W_Interact`) false false)))

(event `close chest`
  (bind _cube (`self.Cube`))
  (bind (_relativerotation_roll _relativerotation_pitch _relativerotation_yaw) (`KismetMathLibrary.BreakRotator` (`SceneComponent.RelativeRotation` _cube)))
  (bind (_direction _chest_float_track) (`Timeline|Chest timeline` :!via `Reverse` :!label _label)
    (:`Update`
      (`SceneComponent.K2_SetRelativeRotation` _cube (`KismetMathLibrary.MakeRotator` _relativerotation_roll (`KismetMathLibrary.Lerp` 0.0 60.0 _chest_float_track) _relativerotation_yaw) false false))))

(event `/Game/CombatFrameWork/Blueprints/Interfaces/BP_Interact.Interact`
  (params (Actor :type "Actor Object Reference") (Inventory :type "/Game/Inventory/Blueprints/BP_Inventory Object Reference"))
  (if (not (`Widget.IsVisible` (`self.LootbarWidget`)))
    (`UserWidget.AddToViewport` (`self.LootbarWidget`) 0)
    (goto _label)))

(event `Remove item`
  (params (index :type Integer))
  (`KismetArrayLibrary.Array_Set` (`self.itemsinchest`) index (make `/Game/Inventory/Structures/S_ItemMaster` (struct))))

(fn `UserConstructionScript`)