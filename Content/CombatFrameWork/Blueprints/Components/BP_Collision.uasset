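; Weapon hit-detection component that traces between two sockets on the assigned weapon each tick while collision is on.
; It sweeps an oriented box from the previous to the current end socket, sized by blade length, to avoid gaps in fast attacks.
; Each new actor hit triggers CallDamageActor once per activation, tracked in AlreadyHit and reset on turn-on.
; An older multi-sphere trace remains disconnected as a fallback.
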(event `Collision Trace`
  (bind _weapon (`self.Weapon`))
  ;[0.01938 0.01938 0.01938] new box trace with no gaps in attacks // https://www.youtube.com/watch?v=NUgCjXI0N-E&ab_channel=JonatanIsaksson
  (set `self.CurrentStartTrace` (`SceneComponent.GetSocketLocation` _weapon (`self.Start Socket`)))
  (set `self.CurrentEndTrace` (`SceneComponent.GetSocketLocation` _weapon (`self.End Socket `)))
  (bind _outhits (`KismetSystemLibrary.BoxTraceMultiForObjects` (`self.Previous End Trace`) (`self.CurrentEndTrace`) (`KismetMathLibrary.MakeVector` (`KismetMathLibrary.Vector_Distance` (`self.CurrentEndTrace`) (`self.CurrentStartTrace`)) (`self.Horizontal collision length`) (`self.VerticalCollisionLength`)) (`KismetMathLibrary.FindLookAtRotation` (`self.CurrentEndTrace`) (`self.CurrentStartTrace`)) (`self.Object Types`) false (`self.Actors to Ignore`) (`self.Draw Debug Type`)))
  (set `self.PreviousStartTrace` (`self.CurrentStartTrace`))
  (set `self.Previous End Trace` (`self.CurrentEndTrace`))
  (for _array_element _outhits
    (bind _output_get (set `self.Last Hit` _array_element))
    (bind (_bblockinghit _binitialoverlap _time _distance _location _impactpoint _normal _impactnormal _physmat _hitactor) (`GameplayStatics.BreakHitResult` _output_get))
    (bind _returnvalue (`self.Can Hit Actor` _hitactor))
    (if _returnvalue
      (bind _output_get_2 (set `self.Hit Actor` _hitactor))
      (`KismetArrayLibrary.Array_Add` (`self.Already Hit ?`) _output_get_2)
      (`self.Damage Actor` (`self.Last Hit`)))))

(event `self.ReceiveTick`
  (params (DeltaSeconds :type "Float (single-precision)"))
  (if (`self.Collision Is On ?`)
    (`self.Collision Trace`)))

(event `Turn On Collision`
  (bind _weapon (`self.Weapon`))
  (`self.Clear Hit Actors`)
  (set `self.Collision Is On ?` true)
  ;[0.01938 0.01938 0.01938] Resets the socket location before activating new collison anim
  (set `self.PreviousStartTrace` (`SceneComponent.GetSocketLocation` _weapon (`self.Start Socket`)))
  (set `self.Previous End Trace` (`SceneComponent.GetSocketLocation` _weapon (`self.End Socket `))))

(event `Clear Hit Actors`
  (`KismetArrayLibrary.Array_Clear` (`self.Already Hit ?`)))

(event `Turn Off Colliison`
  (set `self.Collision Is On ?` false))

(event `Set Weapon`
  (params (Weapon :type "PrimitiveComponent Object Reference"))
  (set `self.Weapon` Weapon))

(fn `Can Hit Actor`
  (params (Actor :type "Actor Object Reference"))
  (returns (ReturnValue :type Boolean))
  (return (not (`KismetArrayLibrary.Array_Contains` (`self.Already Hit ?`) Actor))))