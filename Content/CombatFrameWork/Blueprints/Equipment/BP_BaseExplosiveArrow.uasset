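; Base explosive arrow Blueprint that adds an impact particle effect to the behavior inherited from its parent.
; On actor overlap it runs the parent's handler, then binds SpawnVFX to the VFX event dispatcher.
; When that dispatcher fires, SpawnVFX spawns the VFXOnImpact emitter at the arrow's location.
; The graph itself contains no damage logic and never calls the dispatcher.
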(event `self.ReceiveActorBeginOverlap`
  (params (OtherActor :type "Actor Object Reference"))
  (`parent.ReceiveActorBeginOverlap` OtherActor)
  (add `self.VFX` (delegate `SpawnVFX`)))

(event `SpawnVFX`
  (`GameplayStatics.SpawnEmitterAtLocation` (`self.VFX On Impact`) (`self.K2_GetActorLocation`)))

(fn `UserConstructionScript`
  (`parent.UserConstructionScript`))