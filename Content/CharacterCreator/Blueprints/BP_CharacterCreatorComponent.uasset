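; Character creator component that applies appearance and starting-class choices to its owning Character.
; BeginPlay creates dynamic materials for skin, eyes and hair, and Initialize attaches the supplied hair, beard, moustache, chest and leg components to the body mesh.
; Update events swap gender, hair and gendered class outfit meshes, toggle facial hair, and set colours and facial-marking textures through those materials.
; Sliders drive skin parameters, morph targets, or bone scales in ABP_Manny.
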(event `UpdateHairMaterialInstance`
  (bind _hair (`self.Hair`))
  ; Creating Material Instance References
  (bind _returnvalue (`PrimitiveComponent.CreateDynamicMaterialInstance` _hair 0 (`PrimitiveComponent.GetMaterial` _hair 0) "None" :!label _label))
  (set `self.HairMaterialInstance` _returnvalue))

(event `self.ReceiveBeginPlay`
  (bind _mesh (`self.Mesh`))
  (bind _mesh_2 (`self.Mesh`))
  (bind _mesh_3 (`self.Mesh`))
  ; Creating Material Instance References
  (bind _ascharacter (cast `Character` (`self.GetOwner`)))
  (bind _mesh_4 (`Character.Mesh` _ascharacter))
  (set `self.Mesh` _mesh_4)
  (set `self.AnimationBPRef` (cast `/Game/Characters/Mannequins/Animations/ABP_Manny` (`SkeletalMeshComponent.GetAnimInstance` _mesh_4) :!pure true))
  (bind _returnvalue (`PrimitiveComponent.CreateDynamicMaterialInstance` _mesh 0 (`PrimitiveComponent.GetMaterial` _mesh 0) "None"))
  (set `self.SkinMaterialInstance` _returnvalue)
  (bind _returnvalue_2 (`PrimitiveComponent.CreateDynamicMaterialInstance` _mesh_2 2 (`PrimitiveComponent.GetMaterial` _mesh_2 2) "None"))
  (set `self.RightEyeMaterialInstance` _returnvalue_2)
  (bind _returnvalue_3 (`PrimitiveComponent.CreateDynamicMaterialInstance` _mesh_3 3 (`PrimitiveComponent.GetMaterial` _mesh_3 3) "None"))
  (set `self.LeftEyeMaterialInstance` _returnvalue_3)
  (goto _label))

(event `Update Gender`
  (params (Gender :type "/Game/CharacterCreator/Blueprints/Enums/E_Gender Enum" :default "NewEnumerator0"))
  ; Gender Selector
  (bind _output_get (set `self.Gender` Gender))
  (switch `/Game/CharacterCreator/Blueprints/Enums/E_Gender` _output_get
    (:`NewEnumerator0`
      (`SkeletalMeshComponent.SetSkeletalMeshAsset` (`self.Mesh`) "/Game/CharacterCreator/SkeltalMesh/Male/SK_MaleBase.SK_MaleBase"))
    (:`NewEnumerator1`
      (`SkeletalMeshComponent.SetSkeletalMeshAsset` (`self.Mesh`) "/Game/CharacterCreator/SkeltalMesh/Female/SK_FemaleBase.SK_FemaleBase"))))

(event `UpdateSlider`
  (params (ParameterType :type "/Game/CharacterCreator/Blueprints/Enums/E_ParameterType Enum" :default "NewEnumerator0") (Name :type Name) (Value :type "Float (double-precision)"))
  (bind _animationbpref (`self.AnimationBPRef`))
  (bind _returnvalue (`KismetMathLibrary.Conv_DoubleToVector` (`self.Value`)))
  ; Morph target Silders
  (set `self.Name` Name)
  (set `self.Value` Value)
  (switch `/Game/CharacterCreator/Blueprints/Enums/E_ParameterType` ParameterType
    (:`NewEnumerator0`
      (`MaterialInstanceDynamic.SetScalarParameterValue` (`self.SkinMaterialInstance`) (`self.Name`) (`self.Value`)))
    (:`NewEnumerator1`
      (switch `name` (`self.Name`)
        (:`Head`
          (set `/Game/Characters/Mannequins/Animations/ABP_Manny.HeadScale` _returnvalue _animationbpref))
        (:`Chest`
          (set `/Game/Characters/Mannequins/Animations/ABP_Manny.ChestScale` _returnvalue _animationbpref))
        (:`Abdomen`
          (set `/Game/Characters/Mannequins/Animations/ABP_Manny.AbdomenScale` _returnvalue _animationbpref))
        (:`Legs`
          (set `/Game/Characters/Mannequins/Animations/ABP_Manny.LegsScale` _returnvalue _animationbpref))
        (:`Arms`
          (set `/Game/Characters/Mannequins/Animations/ABP_Manny.ArmsScale` _returnvalue _animationbpref))))
    (:`NewEnumerator2`
      (`SkeletalMeshComponent.SetMorphTarget` (`self.Mesh`) (`self.Name`) (`self.Value`) true))
    (:`NewEnumerator3`
      (`SkeletalMeshComponent.SetMorphTarget` (`self.Beard`) (`self.Name`) (`self.Value`) true))))

(event `AdjustColor`
  (params (Color :type "LinearColor Structure") (Category :type "/Game/CharacterCreator/Blueprints/Enums/E_ColorCategory Enum" :default "NewEnumerator0"))
  ; Colors Sliders
  (set `self.Color` Color)
  (switch `/Game/CharacterCreator/Blueprints/Enums/E_ColorCategory` Category
    (:`NewEnumerator0`
      (`MaterialInstanceDynamic.SetVectorParameterValue` (`self.SkinMaterialInstance`) "Skin_Tint" (`self.Color`)))
    (:`NewEnumerator1`
      (`MaterialInstanceDynamic.SetVectorParameterValue` (`self.RightEyeMaterialInstance`) "Iris Color" (`self.Color`)))
    (:`NewEnumerator2`
      (`MaterialInstanceDynamic.SetVectorParameterValue` (`self.LeftEyeMaterialInstance`) "Iris Color" (`self.Color`)))
    (:`NewEnumerator3`
      (`MaterialInstanceDynamic.SetVectorParameterValue` (`self.HairMaterialInstance`) "Base Color Tint" (`self.Color`)))
    (:`NewEnumerator4`
      (`self.BeardMaterialInstance`
        (:`then`
          (`MaterialInstanceDynamic.SetVectorParameterValue` (`self.BeardMaterialInstance`) "Base Color Tint" (`self.Color`)))
        (:`else`)))
    (:`NewEnumerator5`
      (`self.MoustacheMaterialInstance`
        (:`then`
          (`MaterialInstanceDynamic.SetVectorParameterValue` (`self.MoustacheMaterialInstance`) "Base Color Tint" (`self.Color`)))
        (:`else`)))
    (:`NewEnumerator6`
      (`MaterialInstanceDynamic.SetVectorParameterValue` (`self.SkinMaterialInstance`) "Color Tint" (`self.Color`)))))

(event `UpdateHairStyle`
  (params (NewMesh :type "StaticMesh Object Reference") (HairName :type Name))
  (bind _hair (`self.Hair`))
  ; update hair styles
  (bind _output_get (set `self.Hair Name` HairName))
  (`StaticMeshComponent.SetStaticMesh` _hair NewMesh)
  (switch `name` _output_get
    (:`1`
      (`PrimitiveComponent.SetMaterial` _hair 0 "/Game/CharacterCreator/Hair/male/HairMaterials/1/m_hair_1.m_hair_1")
      (`self.UpdateHairMaterialInstance`))
    (:`2`
      (`PrimitiveComponent.SetMaterial` _hair 0 "/Game/CharacterCreator/Hair/male/HairMaterials/2/m_hair_2.m_hair_2")
      (`self.UpdateHairMaterialInstance`))
    (:`3`
      (`PrimitiveComponent.SetMaterial` _hair 0 "/Game/CharacterCreator/Hair/male/HairMaterials/3/m_hair_3.m_hair_3")
      (`self.UpdateHairMaterialInstance`))
    (:`4`
      (`PrimitiveComponent.SetMaterial` _hair 0 "/Game/CharacterCreator/Hair/male/HairMaterials/4/m_hair_4.m_hair_4")
      (`self.UpdateHairMaterialInstance`))
    (:`5`
      (`PrimitiveComponent.SetMaterial` _hair 0 "/Game/CharacterCreator/Hair/female/Femalehairmaterials/1/F_Hair_1_mt.F_Hair_1_mt")
      (`self.UpdateHairMaterialInstance`))
    (:`6`
      (`PrimitiveComponent.SetMaterial` _hair 0 "/Game/CharacterCreator/Hair/female/Femalehairmaterials/2/F_Hair_2_mt.F_Hair_2_mt")
      (`self.UpdateHairMaterialInstance`))
    (:`7`
      (`PrimitiveComponent.SetMaterial` _hair 0 "/Game/CharacterCreator/Hair/female/Femalehairmaterials/3/F_Hair_3_mt.F_Hair_3_mt")
      (`self.UpdateHairMaterialInstance`))
    (:`8`
      (`PrimitiveComponent.SetMaterial` _hair 0 "/Game/CharacterCreator/Hair/female/Femalehairmaterials/4/F_Hair_4_mt.F_Hair_4_mt")
      (`self.UpdateHairMaterialInstance`))))

(event `ToggleBeard`
  (params (Value :type Boolean))
  (bind _beard (`self.Beard`))
  ; Toggles Facial Hair
  (`SkeletalMeshComponent.SetSkeletalMeshAsset` (`self.Beard`) (select `bool` Value :`true` "/Game/CharacterCreator/Hair/Facialhair/Beard/beard_1_skm.beard_1_skm" :!type "SkeletalMesh Object Reference"))
  ; Creates a valid reference
  (if Value
    (bind _returnvalue (`PrimitiveComponent.CreateDynamicMaterialInstance` _beard 0 (`PrimitiveComponent.GetMaterial` _beard 0) "None"))
    (set `self.BeardMaterialInstance` _returnvalue)
    (else
      (set `self.BeardMaterialInstance` null))))

(event `ToggleMustache`
  (params (Index :type Boolean))
  (bind _moustache (`self.Moustache`))
  ; Toggles Facial Hair
  (`SkeletalMeshComponent.SetSkeletalMeshAsset` (`self.Moustache`) (select `bool` Index :`true` "/Game/CharacterCreator/Hair/Facialhair/moustache/moustache_skm.moustache_skm" :!type "SkeletalMesh Object Reference"))
  ; Creates a valid reference
  (if Index
    (bind _returnvalue (`PrimitiveComponent.CreateDynamicMaterialInstance` _moustache 0 (`PrimitiveComponent.GetMaterial` _moustache 0) "None"))
    (set `self.MoustacheMaterialInstance` _returnvalue)
    (else
      (set `self.MoustacheMaterialInstance` null))))

(event `UpdateFacialMarking`
  (params (FacialMarking :type "Texture2D Object Reference") (FacialNormal :type "Texture2D Object Reference") (Name :type Name))
  (bind _skinmaterialinstance (`self.SkinMaterialInstance`))
  ; Facial markings
  (set `self.FacialMarkingName` Name)
  (`MaterialInstanceDynamic.SetTextureParameterValue` _skinmaterialinstance "Decal Map" FacialMarking)
  (`MaterialInstanceDynamic.SetTextureParameterValue` _skinmaterialinstance "Decal Map Normal" FacialNormal))

(event `UpdatePlayerClass`
  (params (Selection :type String))
  ; Starting Class
  (bind _output_get (set `self.Class` Selection))
  (switch `string` _output_get
    (:`Deprived`
      (`SkeletalMeshComponent.SetSkeletalMeshAsset` (`self.Chest`) null)
      (`SkeletalMeshComponent.SetSkeletalMeshAsset` (`self.Legs`) null))
    (:`Knight`
      (switch `/Game/CharacterCreator/Blueprints/Enums/E_Gender` (`self.Gender`)
        (:`NewEnumerator0`
          (`SkeletalMeshComponent.SetSkeletalMeshAsset` (`self.Chest`) "/Game/CharacterCreator/SkeltalMesh/Outfits/Knight/male/knight_m_body.knight_m_body")
          (`SkeletalMeshComponent.SetSkeletalMeshAsset` (`self.Legs`) "/Game/CharacterCreator/SkeltalMesh/Outfits/Knight/male/knight_m_legs.knight_m_legs"))
        (:`NewEnumerator1`
          (`SkeletalMeshComponent.SetSkeletalMeshAsset` (`self.Chest`) "/Game/CharacterCreator/SkeltalMesh/Outfits/Knight/female/f_knight_body.f_knight_body")
          (`SkeletalMeshComponent.SetSkeletalMeshAsset` (`self.Legs`) "/Game/CharacterCreator/SkeltalMesh/Outfits/Knight/female/f_knight_legs.f_knight_legs"))))
    (:`Wizard`
      (switch `/Game/CharacterCreator/Blueprints/Enums/E_Gender` (`self.Gender`)
        (:`NewEnumerator0`
          (`SkeletalMeshComponent.SetSkeletalMeshAsset` (`self.Chest`) "/Game/CharacterCreator/SkeltalMesh/Outfits/outfits/Wizard/male/m_wizard_body.m_wizard_body")
          (`SkeletalMeshComponent.SetSkeletalMeshAsset` (`self.Legs`) "/Game/CharacterCreator/SkeltalMesh/Outfits/outfits/Wizard/male/m_wizard_bottom.m_wizard_bottom"))
        (:`NewEnumerator1`
          (`SkeletalMeshComponent.SetSkeletalMeshAsset` (`self.Chest`) "/Game/CharacterCreator/SkeltalMesh/Outfits/outfits/Wizard/female/f_wizard_body.f_wizard_body")
          (`SkeletalMeshComponent.SetSkeletalMeshAsset` (`self.Legs`) "/Game/CharacterCreator/SkeltalMesh/Outfits/outfits/Wizard/female/f_wizard_bottom.f_wizard_bottom"))))))

(fn `Initialize`
  (params (Hair :type "StaticMeshComponent Object Reference") (Beard :type "SkeletalMeshComponent Object Reference") (Moustache :type "SkeletalMeshComponent Object Reference") (Chest :type "SkeletalMeshComponent Object Reference") (Legs :type "SkeletalMeshComponent Object Reference"))
  (set `self.Beard` Beard)
  (set `self.Moustache` Moustache)
  (bind _output_get (set `self.Hair` Hair))
  (set `self.Chest` Chest)
  (set `self.Legs` Legs)
  (`SceneComponent.K2_AttachToComponent` _output_get (`self.Mesh`) "None" "SnapToTarget" "SnapToTarget" "SnapToTarget" true)
  (`SceneComponent.K2_AttachToComponent` (`self.Beard`) (`self.Mesh`) "None" "SnapToTarget" "SnapToTarget" "SnapToTarget" true)
  (`SceneComponent.K2_AttachToComponent` (`self.Moustache`) (`self.Mesh`) "None" "SnapToTarget" "SnapToTarget" "SnapToTarget" true)
  (`SceneComponent.K2_AttachToComponent` (`self.Chest`) (`self.Mesh`) "None" "SnapToTarget" "SnapToTarget" "SnapToTarget" true)
  (`SceneComponent.K2_AttachToComponent` (`self.Legs`) (`self.Mesh`) "None" "SnapToTarget" "SnapToTarget" "SnapToTarget" true))