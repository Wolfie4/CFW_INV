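; BP_EquipAN is an anim notify that completes weapon equipping at a point in an animation.
; It finds the owner's BP_Combat component, calls its toggle-equipment function with true, enables combat and attaches the main-hand weapon to its equipped socket.
; A valid off-hand item is also attached to its own equipped socket, but only when the main-hand weapon has one specific combat type.
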(fn `Received_Notify`
  (params (MeshComp :type "SkeletalMeshComponent Object Reference") (Animation :type "AnimSequenceBase Object Reference") (EventReference :type "AnimNotifyEventReference Structure (by ref)"))
  (returns (ReturnValue :type Boolean))
  (bind _returnvalue (`Actor.GetComponentByClass` (`ActorComponent.GetOwner` MeshComp) "/Game/CombatFrameWork/Blueprints/Components/BP_Combat.BP_Combat_C"))
  (bind _mainhandweapon (`/Game/CombatFrameWork/Blueprints/Components/BP_Combat.MainHandWeapon` _returnvalue))
  (bind _mainoffhand (`/Game/CombatFrameWork/Blueprints/Components/BP_Combat.MainOffhand` _returnvalue))
  (`/Game/CombatFrameWork/Blueprints/Components/BP_Combat.ToggleEquipment` _returnvalue true)
  (set `/Game/CombatFrameWork/Blueprints/Components/BP_Combat.CombatEnabled?` true _returnvalue)
  (`/Game/CombatFrameWork/Blueprints/Equipment/BP_BaseEquipment.Attach To Player` _mainhandweapon (`/Game/CombatFrameWork/Blueprints/Equipment/BP_BaseWeapon.EquippedSocket` _mainhandweapon))
  (`/Engine/EditorBlueprintResources/StandardMacros.IsValid` _mainoffhand
    (:`Is Valid`
      (if (`|EnumEquality` (`/Game/CombatFrameWork/Blueprints/Equipment/BP_BaseWeapon.CombatType` _mainhandweapon) "NewEnumerator1")
        (`/Game/CombatFrameWork/Blueprints/Equipment/BP_BaseEquipment.Attach To Player` _mainoffhand (`/Game/CombatFrameWork/Blueprints/Equipment/BP_Offhand.EquippedSocket` _mainoffhand))
        (return true)
        (else
          (return true))))
    (:`Is Not Valid`
      (return true))))