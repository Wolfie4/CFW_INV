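; BP_Money is a world money pickup that adds its Amount to the player's inventory when interacted with.
; A Sphere overlap with the player character shows an outline overlay material on the Money component and reveals the WInteract prompt, and leaving clears both.
; The Interact event increases the inventory's Money, refreshes the WBMoney widget through the inventory, then destroys the actor.
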(event `self.Sphere.OnComponentBeginOverlap`
  (params (OverlappedComponent :type "PrimitiveComponent Object Reference") (OtherActor :type "Actor Object Reference") (OtherComp :type "PrimitiveComponent Object Reference") (OtherBodyIndex :type Integer) (bFromSweep :type Boolean) (SweepResult :type "HitResult Structure (by ref)"))
  (if (== OtherActor (`GameplayStatics.GetPlayerCharacter` 0))
    (`MeshComponent.SetOverlayMaterial` (`self.Money`) "/Game/Inventory/Materials/M_Outline_InstTest.M_Outline_InstTest")
    (`SceneComponent.SetVisibility` (`self.W_Interact`) true false)))

(event `self.Sphere.OnComponentEndOverlap`
  (params (OverlappedComponent :type "PrimitiveComponent Object Reference") (OtherActor :type "Actor Object Reference") (OtherComp :type "PrimitiveComponent Object Reference") (OtherBodyIndex :type Integer))
  (if (== OtherActor (`GameplayStatics.GetPlayerCharacter` 0))
    (`MeshComponent.SetOverlayMaterial` (`self.Money`) null)
    (`SceneComponent.SetVisibility` (`self.W_Interact`) false false)))

(event `/Game/CombatFrameWork/Blueprints/Interfaces/BP_Interact.Interact`
  (params (Actor :type "Actor Object Reference") (Inventory :type "/Game/Inventory/Blueprints/BP_Inventory Object Reference"))
  (set `/Game/Inventory/Blueprints/BP_Inventory.Money` (+ (`/Game/Inventory/Blueprints/BP_Inventory.Money` Inventory) (`self.Amount`)) Inventory)
  (`/Game/Inventory/WidgetBlueprints/WB_Money.UpdateMoney` (`/Game/Inventory/WidgetBlueprints/WB_Inventory.WB_Money` (`/Game/Inventory/Blueprints/BP_Inventory.Inventory` Inventory)))
  (`self.K2_DestroyActor`))

(fn `UserConstructionScript`)