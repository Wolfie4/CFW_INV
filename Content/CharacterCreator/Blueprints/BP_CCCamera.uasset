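; BP_CCCamera is the character creator camera, handling zoom between body and face views and rotation of the referenced character.
; It adds the creator's Enhanced Input mapping context, then uses a rotate action or right-mouse drag to spin the character.
; Scrolling lerps the camera between its starting location and the character's FaceScene.
; MoveCameraToFace and MoveCameraToBody animate the same move with timelines, setting the scroll value to match.
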(event `self.ReceiveBeginPlay`
  (`EnhancedInputSubsystemInterface.AddMappingContext` (pcsubsystem `EnhancedInputLocalPlayerSubsystem` (`GameplayStatics.GetPlayerController` 0)) "/Game/CharacterCreator/Input/CharacterCreatorInputMapping.CharacterCreatorInputMapping" 0 (struct))
  (set `self.StartingCameraLocation` (`self.K2_GetActorLocation`)))

(event `InputAxisKey|MouseX` :consume false
  (params (AxisValue :type "Float (single-precision)"))
  (if (`self.RightMouseButtonDown`)
    (`/Game/CharacterCreator/Blueprints/BP_CharacterCreated.Update Rotation` (`self.CharacterRef`) (* AxisValue -4.0))
    (`KismetSystemLibrary.PrintString` "rotating")))

(event `EnhancedInput|/Game/CharacterCreator/Input/IA_Rotate`
  (params (ActionValue :type "Float (double-precision)") (ElapsedSeconds :type "Float (double-precision)") (TriggeredSeconds :type "Float (double-precision)") (InputAction :type "InputAction Object Reference" :default "/Game/CharacterCreator/Input/IA_Rotate.IA_Rotate"))
  (:`Triggered`
    (`/Game/CharacterCreator/Blueprints/BP_CharacterCreated.Update Rotation` (`self.CharacterRef`) (* ActionValue -4.0))))

(event `EnhancedInput|/Game/CharacterCreator/Input/IA_RightMouseButton`
  (params (ActionValue :type Boolean) (ElapsedSeconds :type "Float (double-precision)") (TriggeredSeconds :type "Float (double-precision)") (InputAction :type "InputAction Object Reference" :default "/Game/CharacterCreator/Input/IA_RightMouseButton.IA_RightMouseButton"))
  (:`Triggered`
    (set `self.RightMouseButtonDown` true)
    (`KismetSystemLibrary.PrintString` "on"))
  (:`Completed`
    (set `self.RightMouseButtonDown` false)
    (`KismetSystemLibrary.PrintString` "off")))

(event `EnhancedInput|/Game/CharacterCreator/Input/IA_Scroll`
  (params (ActionValue :type "Float (double-precision)") (ElapsedSeconds :type "Float (double-precision)") (TriggeredSeconds :type "Float (double-precision)") (InputAction :type "InputAction Object Reference" :default "/Game/CharacterCreator/Input/IA_Scroll.IA_Scroll"))
  (:`Triggered`
    (set `self.Scroll` (`KismetMathLibrary.FClamp` (+ (/ ActionValue 10.0) (`self.Scroll`))))
    (`self.K2_SetActorLocation` (`KismetMathLibrary.VLerp` (`self.StartingCameraLocation`) (`SceneComponent.K2_GetComponentLocation` (`/Game/CharacterCreator/Blueprints/BP_CharacterCreated.FaceScene` (`self.CharacterRef`))) (`self.Scroll`)))))

(event `MoveCameraToFace`
  (bind (_direction _alpha) (`Timeline|Timeline` :!via `PlayFromStart`)
    (:`Update`
      (`self.K2_SetActorLocation` (`KismetMathLibrary.VLerp` (`self.K2_GetActorLocation`) (`SceneComponent.K2_GetComponentLocation` (`/Game/CharacterCreator/Blueprints/BP_CharacterCreated.FaceScene` (`self.CharacterRef`))) _alpha))
      (set `self.Scroll` 1.0))))

(event `MoveCameraToBody`
  (bind (_direction _alpha) (`Timeline|Timeline_0` :!via `PlayFromStart`)
    (:`Update`
      (`self.K2_SetActorLocation` (`KismetMathLibrary.VLerp` (`self.K2_GetActorLocation`) (`self.StartingCameraLocation`) _alpha))
      (set `self.Scroll` 0.0))))

(fn `SetCharacterRef`
  (params (CharacterRef :type "/Game/CharacterCreator/Blueprints/BP_CharacterCreated Object Reference"))
  (set `self.CharacterRef` CharacterRef))

(fn `UserConstructionScript`)